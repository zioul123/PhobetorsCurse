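; PC_ProjectileBase is a projectile actor that deals damage on overlap and plays an impact effect when destroyed.
; Overlapping a PC_CharacterBase other than the Instigator applies fixed damage credited to the Instigator's controller, then destroys the projectile.
; Overlaps with any other actor also destroy it, while overlapping the shooter does nothing.
; The Destroyed event spawns the P_Impulse particle emitter at the projectile's location.
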(event Collision|EventActorBeginOverlap
  (params (OtherActor :type Actor%20Object%20Reference))
  (bind _instigator (Variables|Actor|GetInstigator))
  ;[1 1 1] If the overlapped pawn is not the one who shot it, damage pawn, and destroy projectile
  (bind _aspc_character_base (Utilities|Casting|CastToPC_CharacterBase OtherActor)
    (:then
      (if (not (== _aspc_character_base _instigator))
        (Game|Damage|ApplyDamage _aspc_character_base 5e+01 (Pawn|GetController _instigator) self)
        (Actor|DestroyActor :!label _label)))
    (:CastFailed
      (goto _label))))

(event EventDestroyed
  ;[1 1 1] Play impulse effect
  (Effects|SpawnEmitteratLocation "/Game/Assets/Effects/P_Impulse.P_Impulse" (Transformation|GetActorLocation)))

(fn ConstructionScript)