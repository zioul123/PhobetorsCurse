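; Original game mode, kept in an Old folder, that sets up the player HUD and picks where players spawn.
; On BeginPlay it creates the PC_HUD widget, stores it and adds it to the viewport.
; Its ChoosePlayerStart matches each PlayerStart's tag against the TargetSpawnPoint stored in PC_GameInstance, falling back to the first PlayerStart found if none match.
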(event Custom|CreateHUD
  ;[1 1 1] Create HUD
  (bind _returnvalue (UserInterface|CreateWidget "/Game/Blueprints/UI/Old/OldDialogue/PC_HUD.PC_HUD_C"))
  (bind _output_get (Variables|Default|SetPlayerHUD _returnvalue))
  (UserInterface|Viewport|AddtoViewport _output_get 0))

(event EventBeginPlay
  (CallFunction|CreateHUD))

(event EventTick
  (params (DeltaSeconds :type Float%20%28single-precision%29)))

(fn ConstructionScript)

(fn ChoosePlayerStart
  (params (Player :type Controller%20Object%20Reference))
  (bind _aspc_game_instance (Utilities|Casting|CastToPC_GameInstance (Game|GetGameInstance)))
  (bind _outactors (Actor|GetAllActorsOfClass "/Script/Engine.PlayerStart"))
  (for _array_element _outactors
    (if (Utilities|Name|Equal(Name) (Variables|/Script/Engine.PlayerStart|GetPlayerStartTag _array_element) (Utilities|String|StringToName (Variables|/Game/Blueprints/GameLogic/PC_GameInstance.PC_GameInstance_C|GetTargetSpawnPoint _aspc_game_instance)))
      (return _array_element)))
  (return (Utilities|Array|Get(acopy) _outactors)))