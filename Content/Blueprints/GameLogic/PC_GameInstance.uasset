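; Game instance that tracks stage progression and holds the per-stage map and enemy data that drive each level.
; It resets or increments the stage index, opens the matching map by enum name, and falls back to MainMenu past the last stage.
; SpawnEnemies reads the next 1-indexed enemy entry and spawns configured enemy classes at random navigable points around the first PC_BP_EnemyCentre actor, passing in their stats.
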(fn SetStageto0
  (Variables|PC_LevelManagement|SetCurrentStage 0))

(fn IncrementStage
  (Math|Integer|IncrementInt (Variables|PC_LevelManagement|GetCurrentStage)))

(fn LoadCurrentStage
  (bind _returnvalue (Game|GetPlayerController 0))
  (bind _currentstage (Variables|PC_LevelManagement|GetCurrentStage))
  (bind _levelmapdata (Variables|PC_LevelManagement|GetLevelMapData))
  (bind _output (Utilities|Array|Get(acopy) _levelmapdata _currentstage))
  (bind _returnvalue_2 (Utilities|String|EnumtoString (.map _output)))
  (Development|PrintString (Utilities|String|Append "PC_GameInstance: Loading current stage! " _returnvalue_2))
  (if (< (Variables|PC_LevelManagement|GetCurrentStage) (Utilities|Array|Length (Variables|PC_LevelManagement|GetLevelMapData)))
    (Game|OpenLevel(byName) (Utilities|String|StringToName _returnvalue_2))
    (Input|SetInputModeGameOnly _returnvalue)
    (Variables|/Script/Engine.PlayerController|SetbShowMouseCursor _returnvalue false)
    (else
      (Game|OpenLevel(byName) "MainMenu"))))

(fn LoadNextStage
  (PC_LevelTravelling|IncrementStage)
  (PC_LevelTravelling|LoadCurrentStage))

(fn SpawnEnemies
  (bind _currentstage (Variables|PC_LevelManagement|GetCurrentStage))
  (bind _returnvalue (+ _currentstage 1))
  (if (not (>= _returnvalue (Utilities|Array|Length (Variables|PC_LevelManagement|GetLevelEnemyData))))
    (bind _outactors (Actor|GetAllActorsOfClass "/Game/Blueprints/GameLogic/EnemyData/PC_BP_EnemyCentre.PC_BP_EnemyCentre_C"))
    (for _array_element (.enemyspawninfos (Utilities|Array|Get(acopy) (Variables|PC_LevelManagement|GetLevelEnemyData) _returnvalue))
      (for _index (range 1 (.number _array_element))
        (bind _enemy_class (PCLevelEnemies|EnemyEnumtoEnemyClass (.enemytype _array_element)))
        (bind _randomlocation (Class|NavigationSystemV1|GetRandomLocationinNavigableRadius (Transformation|GetWorldLocation (Variables|/Game/Blueprints/GameLogic/EnemyData/PC_BP_EnemyCentre.PC_BP_EnemyCentre_C|GetDefaultSceneRoot (Utilities|Array|Get(acopy) _outactors))) 5e+02 0 0))
        (Game|SpawnActorfromClass _enemy_class (Math|Transform|MakeTransform _randomlocation "0, 0, 0" "1,1,1") "AdjustIfPossibleButAlwaysSpawn" 0 (.aggrorange _array_element) (.primaryattackdmg _array_element) (.maxhp _array_element) 0)))))

(fn EnemyEnumtoEnemyClass
  (params (Enemy%20Enum :type EEnemies%20Enum :default "SHADOW_KNIGHT"))
  (switch Utilities|FlowControl|Switch|SwitchonEEnemies Enemy%20Enum
    (:SHADOW_KNIGHT
      (return "/Game/Blueprints/Actors/CombatCharacters/PC_BP_ShadowKnight.PC_BP_ShadowKnight_C"))
    (:SHADOW_WIZARD_F
      (return "/Game/Blueprints/Actors/CombatCharacters/PC_BP_ShadowWizard_F.PC_BP_ShadowWizard_F_C"))))