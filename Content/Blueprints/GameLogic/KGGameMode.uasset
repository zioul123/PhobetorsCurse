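; Game mode that runs a wave-based enemy game and creates the player HUD.
; Each wave copies a class list from Waves into a shuffled queue, which a looping timer spawns at random PlayerStarts while IsSpawning is set.
; Destroyed enemies trigger a check that starts the next wave once the queue and PC_AIC_AIBase actors are gone.
; After the last wave, it fires the end-game dispatcher and blends the view to EndCamera.
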(event Custom|SpawnEnemy
  ;[1 1 1] If isSpawning, and queue still has enemies, choose a random spawn point and spawn an enemy of that type, remove from queue and bind onDestroy event.
  (if (Variables|Default|GetIsSpawning)
    (if (> (Utilities|Array|Length (Variables|Default|GetQueue)) 0)
      (bind _outactors (Actor|GetAllActorsOfClass "/Script/Engine.PlayerStart"))
      (bind _returnvalue (AI|SpawnAIFromClass (Utilities|Array|Get(acopy) (Variables|Default|GetQueue)) 0 (Transformation|GetActorLocation (Utilities|Array|Get(acopy) _outactors (Math|Random|RandomInteger (Utilities|Array|Length _outactors)))) (Transformation|GetActorRotation (Utilities|Array|Get(acopy) _outactors (Math|Random|RandomInteger (Utilities|Array|Length _outactors)))) false))
      (Utilities|Array|RemoveIndex (Variables|Default|GetQueue))
      (Game|BindEventtoOnDestroyed _returnvalue (delegate Custom|CheckWaveComplete)))))

(event Custom|StartNewWave
  (bind _waveindex (Variables|Default|GetWaveIndex))
  (bind _waves (Variables|Default|GetWaves))
  ;[1 1 1] Set queue to the Waves[WaveIndex]
  (if (>= _waveindex (Utilities|Array|Length _waves))
    (CallFunction|EndGame)
    (else
      (bind _output_get (Variables|Default|SetQueue (.classtospawn (Utilities|Array|Get(acopy) _waves _waveindex))))
      (Math|Integer|IncrementInt _waveindex
        (:%20%20
          (Utilities|Array|Shuffle _output_get))))))

(event Custom|CheckWaveComplete
  (params (DestroyedActor :type Actor%20Object%20Reference))
  ;[1 1 1] When an enemy is killed, check if the queue is empty and there are no more enemies - then start new wave.
  (if (== (Utilities|Array|Length (Variables|Default|GetQueue)) 0)
    (bind _outactors (Actor|GetAllActorsOfClass "/Game/Blueprints/Controllers/PC_AIC_AIBase.PC_AIC_AIBase_C"))
    (if (== (Utilities|Array|Length _outactors) 0)
      (CallFunction|StartNewWave))))

(event Custom|EndGame
  (Default|CallEndGameDispatcher)
  (Game|Player|SetViewTargetwithBlend (Game|GetPlayerController 0) (Variables|Default|GetEndCamera) 4.0 "VTBlend_Linear" 0.0 true))

(event EventBeginPlay
  ;[1 1 1] Create HUD
  (bind _returnvalue (UserInterface|CreateWidget "/Game/Blueprints/UI/HUD/PC_HUD.PC_HUD_C"))
  (bind _output_get (Variables|Default|SetPlayerHUD _returnvalue))
  (UserInterface|Viewport|AddtoViewport _output_get 0)
  ;[1 1 1] Spawn Enemies
  (CallFunction|StartNewWave)
  (Utilities|Time|SetTimerbyEvent (delegate Custom|SpawnEnemy) 1.0 true))

(event EventTick
  (params (DeltaSeconds :type Float%20%28single-precision%29)))

(fn ConstructionScript)