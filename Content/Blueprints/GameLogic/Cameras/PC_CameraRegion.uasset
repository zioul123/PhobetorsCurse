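; Camera region that hands the view to its own spring-arm camera while the Elina Somnia player character passes through it.
; Overlapping TriggerStart or TriggerEnd toggles the region with a blended view-target switch, while the two ForceEnd volumes always return the view to the character.
; While active, Tick lerps the spring arm toward the character's mesh plus the XY offset captured on activation, provided the character reference is valid.
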(event OnComponentBeginOverlap(TriggerStart)
  (params (OverlappedComponent :type Primitive%20Component%20Object%20Reference) (OtherActor :type Actor%20Object%20Reference) (OtherComp :type Primitive%20Component%20Object%20Reference) (OtherBodyIndex :type Integer) (bFromSweep :type Boolean) (SweepResult :type Hit%20Result%20Structure%20%28by%20ref%29))
  (CallFunction|TriggerRegion OtherActor))

(event OnComponentBeginOverlap(TriggerEnd)
  (params (OverlappedComponent :type Primitive%20Component%20Object%20Reference) (OtherActor :type Actor%20Object%20Reference) (OtherComp :type Primitive%20Component%20Object%20Reference) (OtherBodyIndex :type Integer) (bFromSweep :type Boolean) (SweepResult :type Hit%20Result%20Structure%20%28by%20ref%29))
  (CallFunction|TriggerRegion OtherActor))

(event OnComponentBeginOverlap(ForceEnd)
  (params (OverlappedComponent :type Primitive%20Component%20Object%20Reference) (OtherActor :type Actor%20Object%20Reference) (OtherComp :type Primitive%20Component%20Object%20Reference) (OtherBodyIndex :type Integer) (bFromSweep :type Boolean) (SweepResult :type Hit%20Result%20Structure%20%28by%20ref%29))
  (CallFunction|EndRegion OtherActor))

(event OnComponentBeginOverlap(ForceEnd2)
  (params (OverlappedComponent :type Primitive%20Component%20Object%20Reference) (OtherActor :type Actor%20Object%20Reference) (OtherComp :type Primitive%20Component%20Object%20Reference) (OtherBodyIndex :type Integer) (bFromSweep :type Boolean) (SweepResult :type Hit%20Result%20Structure%20%28by%20ref%29))
  (CallFunction|EndRegion OtherActor))

(event EventBeginPlay)

(event Collision|EventActorBeginOverlap
  (params (OtherActor :type Actor%20Object%20Reference)))

(event EventTick
  (params (DeltaSeconds :type Float%20%28single-precision%29))
  (if (Variables|PC_State|GetisActive)
    (Utilities|IsPlayerAlive
      (:Alive
        (CallFunction|TrackPlayerMovement DeltaSeconds)))))

(fn ConstructionScript)

(fn TriggerRegion
  (params (Overlapped :type Actor%20Object%20Reference%20%28by%20ref%29))
  (bind _returnvalue (Game|GetPlayerController 0))
  (bind _blendtime (Variables|PC_Attributes|GetBlendTime))
  (bind _aspc_bp_elina_somnia (Utilities|Casting|CastToPC_BP_ElinaSomnia Overlapped))
  (if (Variables|PC_State|GetisActive)
    (Variables|PC_State|SetisActive false)
    (Game|Player|SetViewTargetwithBlend _returnvalue _aspc_bp_elina_somnia _blendtime "VTBlend_Linear" 0.0 false)
    (else
      (Variables|PC_State|SetisActive true)
      (Game|Player|SetViewTargetwithBlend _returnvalue self _blendtime "VTBlend_Linear" 0.0 false)
      (Variables|PC_State|SetOffset (Math|Vector|MakeVector (.x (- (Transformation|GetWorldLocation (Variables|Default|GetSpringArm)) (Transformation|GetWorldLocation (Variables|/Script/Engine.Character|GetMesh _aspc_bp_elina_somnia)))) (.y (- (Transformation|GetWorldLocation (Variables|Default|GetSpringArm)) (Transformation|GetWorldLocation (Variables|/Script/Engine.Character|GetMesh _aspc_bp_elina_somnia)))) 0.0))
      (Variables|PC_Temp|SetPlayerCharacter _aspc_bp_elina_somnia))))

(fn EndRegion
  (params (Overlapper :type Actor%20Object%20Reference%20%28by%20ref%29))
  (bind _aspc_bp_elina_somnia (Utilities|Casting|CastToPC_BP_ElinaSomnia Overlapper))
  (Variables|PC_State|SetisActive false)
  (Game|Player|SetViewTargetwithBlend (Game|GetPlayerController 0) _aspc_bp_elina_somnia (Variables|PC_Attributes|GetBlendTime) "VTBlend_Linear" 0.0 false))

(fn TrackPlayerMovement
  (params (DeltaTime :type Float%20%28single-precision%29))
  (Transformation|SetWorldLocation (Variables|Default|GetSpringArm) (Math|Vector|Lerp(Vector) (Transformation|GetWorldLocation (Variables|Default|GetSpringArm)) (+ (Variables|PC_State|GetOffset) (Transformation|GetWorldLocation (Variables|/Script/Engine.Character|GetMesh (Variables|PC_Temp|GetPlayerCharacter)))) DeltaTime) false false))