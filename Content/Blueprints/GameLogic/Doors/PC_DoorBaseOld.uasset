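; Base door actor that moves the player to another level on contact.
; When PC_BP_ElinaSomnia under a player controller overlaps DoorCollision, it stores TargetSpawnPoint in PC_GameInstance, then opens the target level.
; The level name comes from converting the TargetLevel enum value to a string, so enum entries stand in for map names.
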(event OnComponentBeginOverlap(DoorCollision)
  (params (OverlappedComponent :type Primitive%20Component%20Object%20Reference) (OtherActor :type Actor%20Object%20Reference) (OtherComp :type Primitive%20Component%20Object%20Reference) (OtherBodyIndex :type Integer) (bFromSweep :type Boolean) (SweepResult :type Hit%20Result%20Structure%20%28by%20ref%29))
  (Utilities|Casting|CastToPC_BP_ElinaSomnia OtherActor)
  (if (Class|Controller|IsPlayerController (Game|GetInstigatorController OtherActor))
    (bind _aspc_game_instance (Utilities|Casting|CastToPC_GameInstance (Game|GetGameInstance)))
    (Variables|/Game/Blueprints/GameLogic/PC_GameInstance.PC_GameInstance_C|SetTargetSpawnPoint _aspc_game_instance (Variables|PCAttributes|GetTargetSpawnPoint))
    (Game|OpenLevel(byName) (Utilities|String|StringToName (Utilities|String|EnumtoString (Variables|PC_Attributes|GetTargetLevel))))))

(fn ConstructionScript)