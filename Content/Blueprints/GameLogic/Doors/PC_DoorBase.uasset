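; PC_DoorBase is a level exit door that sends the player to the next stage.
; When the player-controlled PC_BP_ElinaSomnia overlaps DoorCollision while the door is enabled, it calls LoadNextStage on PC_GameInstance.
; ActivateDoor and DeactivateDoor set the enabled flag and swap the mesh between open and closed material instances, and FlipDoorState toggles between them.
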(event OnComponentBeginOverlap(DoorCollision)
  (params (OverlappedComponent :type Primitive%20Component%20Object%20Reference) (OtherActor :type Actor%20Object%20Reference) (OtherComp :type Primitive%20Component%20Object%20Reference) (OtherBodyIndex :type Integer) (bFromSweep :type Boolean) (SweepResult :type Hit%20Result%20Structure%20%28by%20ref%29))
  (if (Variables|PC_State|GetIsEnabled)
    (Utilities|Casting|CastToPC_BP_ElinaSomnia OtherActor)
    (if (Class|Controller|IsPlayerController (Game|GetInstigatorController OtherActor))
      (bind _aspc_game_instance (Utilities|Casting|CastToPC_GameInstance (Game|GetGameInstance)))
      (Default|LoadNextStage _aspc_game_instance))))

(fn ConstructionScript)

(fn ActivateDoor
  (Variables|PC_State|SetIsEnabled true)
  (Rendering|Material|SetMaterial (Variables|Default|GetStaticMesh) 0 (Variables|PCReferences|GetOpenDoorMI)))

(fn DeactivateDoor
  (Variables|PC_State|SetIsEnabled false)
  (Rendering|Material|SetMaterial (Variables|Default|GetStaticMesh) 0 (Variables|PC_References|GetClosedDoorMI)))

(fn FlipDoorState
  (if (Variables|PC_State|GetIsEnabled)
    (PC_State|DeactivateDoor)
    (else
      (PC_State|ActivateDoor))))