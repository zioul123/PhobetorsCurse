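; BP_DreamBolt is a combat projectile that damages the PC_Character it overlaps, ignoring its own instigator.
; An overlap applies damage credited to the instigator's controller, then destroys the bolt.
; Overlaps with other actor types and blocking hits destroy it without damage.
; Particle emitters play at spawn and on destruction, so every destroy path shows the impact effect.
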(event Collision|EventHit
  (params (MyComp :type Primitive%20Component%20Object%20Reference) (Other :type Actor%20Object%20Reference) (OtherComp :type Primitive%20Component%20Object%20Reference) (bSelfMoved :type Boolean) (HitLocation :type Vector :default "0, 0, 0") (HitNormal :type Vector :default "0, 0, 0") (NormalImpulse :type Vector :default "0, 0, 0") (Hit :type Hit%20Result%20Structure%20%28by%20ref%29))
  ;[1 1 1] Destroy when hitting walls.
  (Actor|DestroyActor))

(event Collision|EventActorBeginOverlap
  (params (OtherActor :type Actor%20Object%20Reference))
  (bind _instigator (Variables|Actor|GetInstigator))
  ;[1 1 1] Deal damage and destroy if overlapped a PC_Character, otherwise destroy
  (bind _aspc_character (Utilities|Casting|CastToPC_Character OtherActor)
    (:then
      (if (!= _aspc_character _instigator)
        (Game|Damage|ApplyDamage _aspc_character (Variables|Default|GetDmg) (Pawn|GetController _instigator) self)
        (Actor|DestroyActor :!label _label)))
    (:CastFailed
      (goto _label))))

(event EventDestroyed
  ;[1 1 1] When destroyed, play impact emitter.
  (Effects|SpawnEmitteratLocation "/Game/Assets/Effects/DreamBolt/PC_DreamBoltImpact.PC_DreamBoltImpact" (Transformation|GetWorldLocation (Variables|Default|GetMainBody)) "0, 0, 0" "0.500000,0.500000,0.500000"))

(event EventBeginPlay
  ;[1 1 1] When created, play spawn emitter.
  (Effects|SpawnEmitteratLocation "/Game/Assets/Effects/DreamBolt/PC_DreamBoltSpawn.PC_DreamBoltSpawn" (Transformation|GetWorldLocation (Variables|Default|GetSphere)) "0, 0, 0" "0.400000,0.400000,0.400000"))

(fn ConstructionScript)