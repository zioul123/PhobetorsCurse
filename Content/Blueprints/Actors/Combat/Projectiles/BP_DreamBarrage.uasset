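; Dream Barrage combat projectile, a child Blueprint that adds its own spawn and impact particle effects.
; BeginPlay spawns a scaled-down spawn emitter at the Sphere component without calling the parent's BeginPlay.
; Destroyed spawns the impact emitter at MainBody, so it plays whenever the actor is destroyed, whatever the cause.
; The graph adds no movement, overlap or damage logic of its own, and construction defers to the parent.
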(event EventBeginPlay
  (Effects|SpawnEmitteratLocation "/Game/Assets/Effects/Projectiles/PC_DreamBarrageSpawn.PC_DreamBarrageSpawn" (Transformation|GetWorldLocation (Variables|Default|GetSphere)) "0, 0, 0" "0.400000,0.400000,0.400000"))

(event Collision|EventActorBeginOverlap
  (params (OtherActor :type Actor%20Object%20Reference))
  (|CallParentFunction OtherActor) ; This node is disabled and will not be called.\nDrag off pins to build functionality.
)

(event EventTick
  (params (DeltaSeconds :type Float%20%28single-precision%29)))

(event EventDestroyed
  (Effects|SpawnEmitteratLocation "/Game/Assets/Effects/Projectiles/PC_DreamBarrageImpact.PC_DreamBarrageImpact" (Transformation|GetWorldLocation (Variables|Default|GetMainBody)) "0, 0, 0" "0.500000,0.500000,0.500000"))

(fn ConstructionScript
  (|CallParentFunction))