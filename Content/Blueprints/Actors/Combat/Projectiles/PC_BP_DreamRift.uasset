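; Dream Rift is a telegraphed, delayed area attack that damages PC_BP_ElinaSomnia pawns within its radius.
; Each tick it follows an optional target and advances a timer, growing a red disk inside a fixed-size yellow one while both fade in and out on a sine curve.
; When the timer expires, it spawns a radius-scaled particle burst, applies damage through a slightly narrower capsule overlap and destroys itself.
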(event EventBeginPlay
  (Variables|PCTemp|SetRadiusOverHundred (/ (Variables|PC_Attributes|GetRadius) 1e+02))
  (CallFunction|UpdateRedDiskSize)
  (Transformation|SetRelativeScale3D (Variables|Default|GetYellowDisk) (Math|Vector|MakeVector (Variables|PCTemp|GetRadiusOverHundred) (Variables|PCTemp|GetRadiusOverHundred) (Variables|PCTemp|GetRadiusOverHundred))))

(event Collision|EventActorBeginOverlap
  (params (OtherActor :type Actor%20Object%20Reference)))

(event EventTick
  (params (DeltaSeconds :type Float%20%28single-precision%29))
  (bind _defaultsceneroot (Variables|Default|GetDefaultSceneRoot))
  (bind _radius (Variables|PC_Attributes|GetRadius))
  (bind _returnvalue (Transformation|GetWorldLocation _defaultsceneroot))
  (bind _returnvalue_2 (/ _radius 2e+02))
  (CallFunction|IfTargetIsValidFollow)
  (Variables|PC_Temp|SetTimePassedSoFar (Math|Float|Clamp(Float) (+ DeltaSeconds (Variables|PC_Temp|GetTimePassedSoFar)) 0.0 (Variables|PCAttributes|GetDuration)))
  (bind _output_get (Variables|PCTemp|SetDurationFrac (/ (Variables|PC_Temp|GetTimePassedSoFar) (Variables|PCAttributes|GetDuration))))
  (if (>= _output_get 1.0)
    (Effects|SpawnEmitteratLocation "/Game/Assets/Effects/Abilities/PE_DreamRift.PE_DreamRift" _returnvalue "0, 0, 0" (Math|Vector|MakeVector _returnvalue_2 _returnvalue_2 _returnvalue_2))
    (bind _outactors (Collision|CapsuleOverlapActors _returnvalue (- (Variables|PC_Attributes|GetRadius) 3e+01) 5e+02 (Utilities|Array|MakeArray "ObjectTypeQuery3") "/Game/Blueprints/Actors/CombatCharacters/PC_BP_ElinaSomnia.PC_BP_ElinaSomnia_C"))
    (for _array_element _outactors
      (Game|Damage|ApplyDamage _array_element (Variables|PCAttributes|GetDamage) 0 0))
    (Actor|DestroyActor)
    (else
      (CallFunction|UpdateDiskOpacities)
      (CallFunction|UpdateRedDiskSize))))

(fn ConstructionScript)

(fn UpdateDiskOpacities
  (bind _durationfrac (Variables|PCTemp|GetDurationFrac))
  (bind _returnvalue (Math|Float|MultiplybyPi _durationfrac))
  (bind _returnvalue_2 (Math|Trig|Sin(Radians) _returnvalue))
  (Rendering|Material|SetScalarParameterValueonMaterials (Variables|Default|GetYellowDisk) "Opacity" (* _returnvalue_2 0.3))
  (Rendering|Material|SetScalarParameterValueonMaterials (Variables|Default|GetRedDisk) "Opacity" (* _returnvalue_2 0.5)))

(fn UpdateRedDiskSize
  (bind _durationfrac (Variables|PCTemp|GetDurationFrac))
  (bind _radiusoverhundred (Variables|PCTemp|GetRadiusOverHundred))
  (bind _returnvalue (* _radiusoverhundred _durationfrac))
  (Transformation|SetRelativeScale3D (Variables|Default|GetRedDisk) (Math|Vector|MakeVector _returnvalue _returnvalue _returnvalue)))

(fn IfTargetIsValidFollow
  (Utilities|IsValid (Variables|PCAttributes|GetFollowTarget)
    (:Is%20Valid
      (Transformation|SetWorldLocation (Variables|Default|GetDefaultSceneRoot) (Transformation|GetWorldLocation (Variables|/Script/Engine.Character|GetMesh (Variables|PCAttributes|GetFollowTarget))) false false))))