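; PC_BP_DreamFlurry is a timed area indicator for a combat projectile, built from a yellow disk and a red disk.
; Each tick advances a normalized duration fraction that scales the red disk linearly toward the configured radius.
; The same fraction drives a sine curve that fades both disks' material opacity in and out.
; At full duration the actor prints an explosion debug message and destroys itself, applying no damage.
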(event EventBeginPlay
  (CallFunction|UpdateRedDiskSize)
  (Variables|PCTemp|SetRadiusOverHundred (/ (Variables|PC_Attributes|GetRadius) 1e+02)))

(event Collision|EventActorBeginOverlap
  (params (OtherActor :type Actor%20Object%20Reference)))

(event EventTick
  (params (DeltaSeconds :type Float%20%28single-precision%29))
  (Variables|PC_Temp|SetTimePassedSoFar (Math|Float|Clamp(Float) (+ DeltaSeconds (Variables|PC_Temp|GetTimePassedSoFar)) 0.0 (Variables|PCAttributes|GetDuration)))
  (bind _output_get (Variables|PCTemp|SetDurationFrac (/ (Variables|PC_Temp|GetTimePassedSoFar) (Variables|PCAttributes|GetDuration))))
  (if (>= _output_get 1.0)
    (Development|PrintString "PC_BP_DreamFlurry::Explosion!")
    (Actor|DestroyActor)
    (else
      (CallFunction|UpdateDiskOpacities)
      (CallFunction|UpdateRedDiskSize))))

(fn ConstructionScript)

(fn UpdateDiskOpacities
  (bind _durationfrac (Variables|PCTemp|GetDurationFrac))
  (bind _returnvalue (Math|Float|MultiplybyPi _durationfrac))
  (bind _returnvalue_2 (Math|Trig|Sin(Radians) _returnvalue))
  (Rendering|Material|SetScalarParameterValueonMaterials (Variables|Default|GetYellowDisk) "Opacity" _returnvalue_2)
  (Rendering|Material|SetScalarParameterValueonMaterials (Variables|Default|GetRedDisk) "Opacity" _returnvalue_2))

(fn UpdateRedDiskSize
  (bind _durationfrac (Variables|PCTemp|GetDurationFrac))
  (bind _radiusoverhundred (Variables|PCTemp|GetRadiusOverHundred))
  (bind _returnvalue (* _radiusoverhundred _durationfrac))
  (Transformation|SetRelativeScale3D (Variables|Default|GetRedDisk) (Math|Vector|MakeVector _returnvalue _returnvalue _returnvalue)))