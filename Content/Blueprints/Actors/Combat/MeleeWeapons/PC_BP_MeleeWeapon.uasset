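; Enemy melee weapon actor that damages only Elina Somnia, the player character, in an area around the sword.
; TryDealDamage requires the attach parent's owner to be a PC_BP_Enemy, then sphere-overlaps Pawns at the sword mesh, filtered to PC_BP_ElinaSomnia.
; Each hit takes the enemy's primary attack damage, with that enemy as damage causer.
; A debug sphere draws the attack radius on every attempt that passes the owner check.
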(event EventTryDealDamage
  (bind _swordmesh (Variables|Default|GetSwordMesh))
  (bind _aoerange (Variables|Default|GetAOERange))
  (bind _returnvalue (Transformation|GetWorldLocation _swordmesh))
  ;[1 1 1] Deal damage in an AOE around the sword to ONLY ELINA SOMNIA nearby. Basic melee weapon should only be used by enemies, and only attacks Elina.
  (bind _aspc_bp_enemy (Utilities|Casting|CastToPC_BP_Enemy (Components|GetOwner (Transformation|GetAttachParent (Variables|Default|GetDefaultSceneRoot)))))
  (Rendering|Debug|DrawDebugSphere _returnvalue _aoerange 12 "(R=1.000000,G=1.000000,B=1.000000,A=1.000000)" 1.0)
  (bind _outactors (Collision|SphereOverlapActors _returnvalue _aoerange (Utilities|Array|MakeArray "ObjectTypeQuery3") "/Game/Blueprints/Actors/CombatCharacters/PC_BP_ElinaSomnia.PC_BP_ElinaSomnia_C"))
  (for _array_element _outactors
    (Game|Damage|ApplyDamage _array_element (Variables|/Game/Blueprints/Actors/CombatCharacters/PC_BP_Enemy.PC_BP_Enemy_C|GetPrimaryAttackDmg _aspc_bp_enemy) 0 _aspc_bp_enemy)))

(fn ConstructionScript)