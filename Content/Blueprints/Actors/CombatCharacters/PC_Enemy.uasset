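; PC_Enemy is an enemy combat character that starts with full health and has a placeholder primary attack for child classes to override.
; BeginPlay calls the parent, then resets HP and MP.
; When damaged while not aggroed, it restarts its PC_AIC_AIBase controller's behavior tree so it tries to aggro again.
; Tick, construction and KillCharacter add nothing beyond the parent logic.
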(event Custom|TryPrimaryAttack
  (Development|PrintString "PC_Enemy:TryPrimaryAttack. Override this event."))

(event EventBeginPlay
  ;[1 1 1] Enemies always spawn with full health.
  (|CallParentFunction)
  (CallFunction|ResetHPMP))

(event Collision|EventActorBeginOverlap
  (params (OtherActor :type Actor%20Object%20Reference)))

(event EventTick
  (params (DeltaSeconds :type Float%20%28single-precision%29))
  (|CallParentFunction DeltaSeconds) ; This node is disabled and will not be called.\nDrag off pins to build functionality.
)

(event Game|Damage|EventAnyDamage
  (params (Damage :type Float%20%28single-precision%29) (DamageType :type Damage%20Type%20Object%20Reference) (InstigatedBy :type Controller%20Object%20Reference) (DamageCauser :type Actor%20Object%20Reference))
  ;[1 1 1] If not currently aggroed but got attacked, try aggro again.
  (|CallParentFunction Damage DamageType InstigatedBy DamageCauser)
  (if (not (Variables|PCState|GetCurrentlyAggro))
    (bind _aspc_aic_aibase (Utilities|Casting|CastToPC_AIC_AIBase (AI|GetAIController self)))
    (AI|Logic|StopLogic (Variables|/Script/AIModule.AIController|GetBrainComponent _aspc_aic_aibase) "")
    (AI|RunBehaviorTree _aspc_aic_aibase (Variables|/Game/Blueprints/Controllers/Common/PC_AIC_AIBase.PC_AIC_AIBase_C|GetBehaviorTree _aspc_aic_aibase))))

(fn ConstructionScript
  (|CallParentFunction))

(fn KillCharacter
  (|CallParentFunction))