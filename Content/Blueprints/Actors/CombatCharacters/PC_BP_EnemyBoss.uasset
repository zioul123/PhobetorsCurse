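; Boss enemy combat character base that acquires Elina Somnia as its target and turns to face her while attacking.
; GetTarget takes the first PC_BP_ElinaSomnia actor in the level on BeginPlay, and Tick retries whenever that target is invalid.
; Autoattack, NextAttack, AbilityDone and the Dream Barrage and Dream Rift handlers are placeholders that only print debug strings.
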(event Custom|TryDreamBarrage
  (Development|PrintString "PC_BP_EnemyBoss::TryDreamBarrage"))

(event Custom|TryDreamRift
  (Development|PrintString "PC_BP_EnemyBoss::TryDreamFlurry"))

(event EventBeginPlay
  (|CallParentFunction)
  (PC_General|GetTarget))

(event Collision|EventActorBeginOverlap
  (params (OtherActor :type Actor%20Object%20Reference))
  (|CallParentFunction OtherActor) ; This node is disabled and will not be called.\nDrag off pins to build functionality.
)

(event EventTick
  (params (DeltaSeconds :type Float%20%28single-precision%29))
  (|CallParentFunction DeltaSeconds)
  (Utilities|IsValid (Variables|PC_References|GetTargetEnemy)
    (:Is%20Valid
      _)
    (:Is%20Not%20Valid
      (PC_General|GetTarget)))
  (PCGeneral|RotatetoTargetifAttacking))

(fn ConstructionScript
  (|CallParentFunction))

(fn FireAutoattack
  (params (AttackingHand :type LRHand%20Enum :default "NewEnumerator0"))
  (Development|PrintString "EnemyBoss::FireAutoattack"))

(fn NextAttack
  (Development|PrintString "EnemyBoss::NextAttack"))

(fn FireDreamRift
  (Development|PrintString "EnemyBoss::FireDreamRift"))

(fn FireDreamBarrage
  (Development|PrintString "EnemyBoss::FireDreamBarrage"))

(fn AbilityDone
  (Development|PrintString "EnemyBoss::AbilityDone"))

(fn GetTarget
  (bind _outactors (Actor|GetAllActorsOfClass "/Game/Blueprints/Actors/CombatCharacters/PC_BP_ElinaSomnia.PC_BP_ElinaSomnia_C"))
  (Variables|PC_References|SetTargetEnemy (Utilities|Array|Get(acopy) _outactors)))

(fn RotatetoTargetifAttacking
  (if (Variables|Default|GetAttackingNow)
    (CallFunction|RotatetoTarget (Variables|PC_References|GetTargetEnemy))))