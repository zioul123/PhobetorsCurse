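; Shadow Knight melee combat character that spawns a weapon actor at BeginPlay and attaches it to its weapon socket.
; Primary attack plays a montage, and an animation-blueprint call asks the weapon to deal damage through the melee weapon interface.
; Both are gated by a check that blocks actions when dead or while the game state reports dialog playing.
; Death disables collision, plays a random death montage, notifies the game state, then destroys character and weapon.
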(event Custom|MeleeDealDamage
  (bind _weapon (Variables|PCReferences|GetWeapon))
  ;[1 1 1] Get the weapon to deal damage (called by animation blueprint)
  (Utilities|IsActionAllowed
    (:True
      (if (Utilities|DoesObjectImplementInterface _weapon "/Game/Blueprints/Weapons/PC_I_MeleeWeapon.PC_I_MeleeWeapon_C")
        (Class|PCIMeleeWeapon|TryDealDamage(Message) _weapon)))))

(event Custom|PlayDeathAnimThenDestroy
  ;[1 1 1] Choose a random death anim montage to play then destroy the actor
  (bind _deathanimmontage (CallFunction|ChooseRandomDeathMontage))
  (bind _returnvalue (Animation|PlayAnimMontage _deathanimmontage 1.0 "None"))
  (Utilities|FlowControl|Delay _returnvalue)
  (Actor|DestroyActor)
  (Actor|DestroyActor (Variables|PCReferences|GetWeapon)))

(event Custom|CreateWeapon
  ;[1 1 1] Create a weapon mesh and attach it to the weapon socket
  (bind _returnvalue (Game|SpawnActorfromClass "/Game/Blueprints/Actors/Combat/MeleeWeapons/PC_BP_MeleeWeapon.PC_BP_MeleeWeapon_C" (Transformation|GetActorTransform) "Undefined" 0 0))
  (bind _output_get (Variables|PCReferences|SetWeapon _returnvalue))
  (Transformation|AttachComponentToComponent _output_get (Variables|Character|GetMesh) "Weapon" "SnapToTarget" "SnapToTarget" "SnapToTarget" false))

(event EventBeginPlay
  (|CallParentFunction)
  (CallFunction|CreateWeapon))

(event Collision|EventActorBeginOverlap
  (params (OtherActor :type Actor%20Object%20Reference)))

(event EventTick
  (params (DeltaSeconds :type Float%20%28single-precision%29))
  (|CallParentFunction DeltaSeconds) ; This node is disabled and will not be called.\nDrag off pins to build functionality.
)

(event EventTryPrimaryAttack
  ;[1 1 1] Start the default melee attack
  (Utilities|IsActionAllowed
    (:True
      (Animation|PlayAnimMontage "/Game/Assets/Characters/Knight/Animations/AM_KG_Attack_PrimaryA.AM_KG_Attack_PrimaryA" 1.0 "None"))))

(fn ConstructionScript
  (|CallParentFunction))

(fn KillCharacter
  (CallFunction|DisableCollisions)
  (CallFunction|PlayDeathAnimThenDestroy)
  (CallFunction|NotifyDeathtoGameState))

(fn ChooseRandomDeathMontage
  (switch int (Math|Random|RandomIntegerinRange 0 3)
    (:0
      (LocalVariables|SetSelectedAnimMontage "/Game/Assets/Characters/Knight/Animations/AM_KG_Death_1_Montage.AM_KG_Death_1_Montage"))
    (:1
      (LocalVariables|SetSelectedAnimMontage "/Game/Assets/Characters/Knight/Animations/AM_KG_Death_2_Montage.AM_KG_Death_2_Montage"))
    (:2
      (LocalVariables|SetSelectedAnimMontage "/Game/Assets/Characters/Knight/Animations/AM_KG_Death_3_Montage.AM_KG_Death_3_Montage"))
    (:3
      (LocalVariables|SetSelectedAnimMontage "/Game/Assets/Characters/Knight/Animations/AM_KG_Death_Fwd_Montage.AM_KG_Death_Fwd_Montage")))
  (return (LocalVariables|GetSelectedAnimMontage)))