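; Elina Stalker enemy character that floats after its target and can kill Elina with a Dream Rift.
; While stalking is active, Tick moves the capsule directly without sweep, adds a sine bob, turns it and eases animation velocity.
; Elina entering the kill-range sphere restarts the AI behavior tree; KillElina freezes her through the game state's dialog flag.
; It also has montage-based attacks, hand-fired Dream Bolts and randomized death animations.
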(event OnComponentBeginOverlap(Sphere)
  (params (OverlappedComponent :type Primitive%20Component%20Object%20Reference) (OtherActor :type Actor%20Object%20Reference) (OtherComp :type Primitive%20Component%20Object%20Reference) (OtherBodyIndex :type Integer) (bFromSweep :type Boolean) (SweepResult :type Hit%20Result%20Structure%20%28by%20ref%29))
  (Utilities|Casting|CastToPC_BP_ElinaSomnia OtherActor)
  (bind _aspc_aic_aibase (Utilities|Casting|CastToPC_AIC_AIBase (AI|GetAIController self)))
  (AI|Logic|StopLogic (Variables|/Script/AIModule.AIController|GetBrainComponent _aspc_aic_aibase) "")
  (AI|RunBehaviorTree _aspc_aic_aibase (Variables|/Game/Blueprints/Controllers/Common/PC_AIC_AIBase.PC_AIC_AIBase_C|GetBehaviorTree _aspc_aic_aibase)))

(event Custom|StalkTarget
  (Variables|PC_State|SetActive true)
  (Development|PrintString "Stalking!"))

(event Custom|PlayDeathAnimThenDestroy
  ;[1 1 1] Choose a random death anim montage to play then destroy the actor
  (bind _deathanimmontage (CallFunction|ChooseRandomDeathMontage))
  (bind _returnvalue (Animation|PlayAnimMontage _deathanimmontage 1.0 "None"))
  (Utilities|FlowControl|Delay _returnvalue)
  (Actor|DestroyActor))

(event Custom|EndStalking
  (Variables|PC_State|SetActive false)
  (Development|PrintString "Unstalking!"))

(event EventBeginPlay
  (|CallParentFunction)
  (CallFunction|GetTarget)
  (Components|Sphere|SetSphereRadius (Variables|Default|GetSphere) (Variables|PC_Attributes|GetKillRange) true))

(event Collision|EventActorBeginOverlap
  (params (OtherActor :type Actor%20Object%20Reference)))

(event EventTick
  (params (DeltaSeconds :type Float%20%28single-precision%29))
  (|CallParentFunction DeltaSeconds)
  (PCStalking|UpdateHeight DeltaSeconds)
  (Utilities|IsValid (Variables|Default|GetTargetEnemy)
    (:Is%20Valid
      _)
    (:Is%20Not%20Valid
      (CallFunction|GetTarget)))
  (if (Variables|PC_State|GetActive)
    (PC_Stalking|MovetoTarget DeltaSeconds)
    (CallFunction|RotatetoTarget (Variables|Default|GetTargetEnemy)))
  (PCStalking|UpdateAnimBPVelocity DeltaSeconds))

(event EventTryPrimaryAttack
  ;[1 1 1] Start the default magic attack
  (CallFunction|SpawnFrontPL)
  (Utilities|RotateforDuration 0.5
    (:Out
      (CallFunction|DeleteAllPLs)
      (Utilities|IsActionAllowed
        (:True
          (Animation|PlayAnimMontage "/Game/Assets/Characters/Common/ES_Animations/AM_M_Primary_Attack_B_Medium_UpperBody.AM_M_Primary_Attack_B_Medium_UpperBody" 1.0 "None"))))))

(fn ConstructionScript
  (|CallParentFunction))

(fn KillCharacter
  (CallFunction|DeleteAllPLs)
  (CallFunction|DisableCollisions)
  (CallFunction|PlayDeathAnimThenDestroy)
  (CallFunction|NotifyDeathtoGameState))

(fn ChooseRandomDeathMontage
  (switch int (Math|Random|RandomIntegerinRange 0 3)
    (:0
      (LocalVariables|SetSelectedAnimMontage "/Game/Assets/Characters/Common/ES_Animations/AM_ES_Death1.AM_ES_Death1"))
    (:1
      (LocalVariables|SetSelectedAnimMontage "/Game/Assets/Characters/Common/ES_Animations/AM_ES_Death2.AM_ES_Death2"))
    (:2
      (LocalVariables|SetSelectedAnimMontage "/Game/Assets/Characters/Common/ES_Animations/AM_ES_Death3.AM_ES_Death3"))
    (:3
      (LocalVariables|SetSelectedAnimMontage "/Game/Assets/Characters/Common/ES_Animations/AM_ES_Death_Fwd_Montage.AM_ES_Death_Fwd_Montage")))
  (return (LocalVariables|GetSelectedAnimMontage)))

(fn FireAutoattack
  (params (AttackingHand :type LRHand%20Enum :default "NewEnumerator0"))
  (bind _mesh (Variables|Character|GetMesh))
  (bind _attackscale (Variables|PC_Attributes|GetAttackScale))
  (switch Utilities|FlowControl|Switch|SwitchonLRHand AttackingHand
    (:NewEnumerator0
      (CallFunction|SpawnDreamBolt (Transformation|GetSocketLocation _mesh "hand_l") _attackscale))
    (:NewEnumerator1
      (CallFunction|SpawnDreamBolt (Transformation|GetSocketLocation _mesh "hand_r") _attackscale)))
  (Development|PrintString "Firing Dream Bolt"))

(fn NextAttack)

(fn MovetoTarget
  (params (DeltaTime :type Float%20%28single-precision%29))
  (bind _targetenemy (Variables|Default|GetTargetEnemy))
  (bind _capsulecomponent (Variables|Default|GetCapsuleComponent))
  (bind _capsulecomponent_2 (Variables|Default|GetCapsuleComponent))
  (bind _returnvalue (Transformation|GetWorldLocation _capsulecomponent_2))
  (bind _returnvalue_2 (Transformation|GetWorldLocation _capsulecomponent))
  (bind _capsulecomponent_3 (Variables|/Script/Engine.Character|GetCapsuleComponent _targetenemy))
  (bind _returnvalue_3 (Transformation|GetWorldLocation _capsulecomponent_3))
  ;[1 1 1] Move her toward Elina
  (Transformation|AddWorldOffset (Variables|Default|GetCapsuleComponent) (* (- _returnvalue_3 _returnvalue) (* DeltaTime (/ (Variables|Default|GetWalkSpeed) (Math|Vector|Distance(Vector) _returnvalue_3 _returnvalue)))) false false)
  ;[1 1 1] Make her wave up and down
  (Transformation|SetWorldLocation _capsulecomponent (Math|Vector|MakeVector (.x _returnvalue_2) (.y _returnvalue_2) (+ (Variables|PCState|GetCurrentHeight) (.z _returnvalue_2))) false false))

(fn UpdateAnimBPVelocity
  (params (DeltaTime :type Float%20%28single-precision%29))
  (bind _returnvalue (* DeltaTime 3.0))
  (if (Variables|PC_State|GetActive)
    (Variables|PCState|SetCurrVelocity (Math|Float|Lerp (Variables|PCState|GetCurrVelocity) (Variables|Default|GetWalkSpeed) _returnvalue))
    (else
      (Variables|PCState|SetCurrVelocity (Math|Float|Lerp (Variables|PCState|GetCurrVelocity) 0.0 _returnvalue)))))

(fn UpdateHeight
  (params (DeltaTime :type Float%20%28single-precision%29))
  (bind _output_get (Variables|PCState|SetHeightFactor (+ DeltaTime (Variables|PCState|GetHeightFactor))))
  (Variables|PCState|SetCurrentHeight (+ (* (Variables|PCAttributes|GetMaxOscilHeight) (Math|Trig|Sin(Radians) (* _output_get (* (* (Math|Trig|GetPI) 2.0) (Variables|PCAttributes|GetOscillationRate))))) (Variables|PCAttributes|GetMaxOscilHeight))))

(fn KillElina
  (bind _targetenemy (Variables|Default|GetTargetEnemy))
  (bind _mesh (Variables|/Script/Engine.Character|GetMesh _targetenemy))
  (bind _returnvalue (Transformation|GetWorldTransform _mesh))
  (bind _aspc_game_state (Utilities|Casting|CastToPC_GameState (Game|GetGameState)))
  (Variables|/Game/Blueprints/GameLogic/PC_GameState.PC_GameState_C|SetIsDialogPlaying _aspc_game_state true) ; This is a hacky way to stop Elina from moving.
  (Game|SpawnActorfromClass "/Game/Blueprints/Actors/Combat/Projectiles/PC_BP_DreamRift.PC_BP_DreamRift_C" (Math|Transform|MakeTransform (Math|Vector|MakeVector (.x (.location _returnvalue)) (.y (.location _returnvalue)) (+ (.z (.location _returnvalue)) 1.0)) (.rotation _returnvalue) "1,1,1") "AlwaysSpawn" 0 1e+02 1.133 1e+03 self)
  (Animation|PlayAnimMontage "/Game/Assets/Characters/Common/ES_Animations/AM_ES_M_CosmicRift_Start_UpperBody.AM_ES_M_CosmicRift_Start_UpperBody" 1.0 "None"))