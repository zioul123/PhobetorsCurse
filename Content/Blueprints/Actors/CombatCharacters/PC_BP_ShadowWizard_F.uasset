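; Combat character Blueprint for the female Shadow Wizard, which faces its target enemy while attacking and performs a magic primary attack.
; Tick reacquires a missing target, while a timed macro flags the attack rotation window.
; The attack spawns a front PL, then after the delay clears PLs and plays its montage if alive and no dialog is playing.
; Death disables collisions, notifies GameState and plays a random montage before destroying the actor.
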(event Custom|PlayDeathAnimThenDestroy
  ;[1 1 1] Choose a random death anim montage to play then destroy the actor
  (bind _deathanimmontage (CallFunction|ChooseRandomDeathMontage))
  (bind _returnvalue (Animation|PlayAnimMontage _deathanimmontage 1.0 "None"))
  (Utilities|FlowControl|Delay _returnvalue)
  (Actor|DestroyActor))

(event EventBeginPlay
  (|CallParentFunction))

(event Collision|EventActorBeginOverlap
  (params (OtherActor :type Actor%20Object%20Reference)))

(event EventTick
  (params (DeltaSeconds :type Float%20%28single-precision%29))
  (|CallParentFunction DeltaSeconds)
  (Utilities|IsValid (Variables|Default|GetTargetEnemy)
    (:Is%20Valid
      _)
    (:Is%20Not%20Valid
      (CallFunction|GetTarget)))
  (CallFunction|RotatetoTargetifAttacking))

(event EventTryPrimaryAttack
  ;[1 1 1] Start the default magic attack
  (CallFunction|SpawnFrontPL)
  (Utilities|RotateforDuration 0.5
    (:Out
      (CallFunction|DeleteAllPLs)
      (Utilities|IsActionAllowed
        (:True
          (Animation|PlayAnimMontage "/Game/Assets/Characters/Common/ES_Animations/AM_M_Primary_Attack_B_Medium.AM_M_Primary_Attack_B_Medium" 1.0 "None"))))))

(fn ConstructionScript
  (|CallParentFunction))

(fn KillCharacter
  (CallFunction|DisableCollisions)
  (CallFunction|PlayDeathAnimThenDestroy)
  (CallFunction|NotifyDeathtoGameState))

(fn ChooseRandomDeathMontage
  (switch int (Math|Random|RandomIntegerinRange 0 3)
    (:0
      (LocalVariables|SetSelectedAnimMontage "/Game/Assets/Characters/Knight/Animations/AM_KG_Death_1_Montage.AM_KG_Death_1_Montage"))
    (:1
      (LocalVariables|SetSelectedAnimMontage "/Game/Assets/Characters/Knight/Animations/AM_KG_Death_2_Montage.AM_KG_Death_2_Montage"))
    (:2
      (LocalVariables|SetSelectedAnimMontage "/Game/Assets/Characters/Knight/Animations/AM_KG_Death_3_Montage.AM_KG_Death_3_Montage"))
    (:3
      (LocalVariables|SetSelectedAnimMontage "/Game/Assets/Characters/Knight/Animations/AM_KG_Death_Fwd_Montage.AM_KG_Death_Fwd_Montage")))
  (return (LocalVariables|GetSelectedAnimMontage)))