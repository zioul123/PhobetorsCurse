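; Shadow Knight combat character Blueprint that adds its own death behavior on top of a parent character class.
; Its KillCharacter override replaces the parent's logic, which is left unconnected, with a call to PlayDeathAnimThenDestroy.
; That event plays one of four death montages at random, waits for the returned montage length, then destroys the actor.
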(event Custom|PlayDeathAnimThenDestroy
  ;[1 1 1] Choose a random death anim montage to play then destroy the actor
  (switch int (Math|Random|RandomIntegerinRange 0 3)
    (:0
      (bind _returnvalue (Animation|PlayAnimMontage "/Game/Assets/Characters/Knight/Animations/AM_KG_Death_1_Montage.AM_KG_Death_1_Montage" 1.0 "None"))
      (Utilities|FlowControl|Delay _returnvalue))
    (:1
      (bind _returnvalue_2 (Animation|PlayAnimMontage "/Game/Assets/Characters/Knight/Animations/AM_KG_Death_2_Montage.AM_KG_Death_2_Montage" 1.0 "None"))
      (Utilities|FlowControl|Delay _returnvalue_2))
    (:2
      (bind _returnvalue_3 (Animation|PlayAnimMontage "/Game/Assets/Characters/Knight/Animations/AM_KG_Death_3_Montage.AM_KG_Death_3_Montage" 1.0 "None"))
      (Utilities|FlowControl|Delay _returnvalue_3))
    (:3
      (bind _returnvalue_4 (Animation|PlayAnimMontage "/Game/Assets/Characters/Knight/Animations/AM_KG_Death_Fwd_Montage.AM_KG_Death_Fwd_Montage" 1.0 "None"))
      (Utilities|FlowControl|Delay _returnvalue_4)))
  (Actor|DestroyActor))

(event EventBeginPlay
  (|CallParentFunction))

(event Collision|EventActorBeginOverlap
  (params (OtherActor :type Actor%20Object%20Reference)))

(event EventTick
  (params (DeltaSeconds :type Float%20%28single-precision%29))
  (|CallParentFunction DeltaSeconds) ; This node is disabled and will not be called.\nDrag off pins to build functionality.
)

(fn ConstructionScript
  (|CallParentFunction))

(fn KillCharacter
  (CallFunction|PlayDeathAnimThenDestroy))