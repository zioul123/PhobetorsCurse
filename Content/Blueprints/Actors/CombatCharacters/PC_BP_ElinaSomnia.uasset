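; Elina Somnia combat character with an automatic Dream Bolt attack, MP-costed Blink and double jump, and random death montages.
; While alive and stationary, Tick targets the nearest living PC_Character in range, preferring line of sight, and loops four attack montages.
; Anim notifies chain attacks and fire bolts from either hand; movement resets the attack.
; Game instance holds ability unlocks and MP costs; Blink teleports forward, stopping at blocking static objects.
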(event Custom|FindClosestTarget
  ;[0 1 0.476] FindClosestTarget: Reset Target, then find the closest living PC_Character with LOS and assign that to Target. If none have LOS, pick closest.
  (Variables|PCState|SetTarget 0)
  (bind (_outactors _returnvalue) (Collision|SphereOverlapActors (Transformation|GetWorldLocation (Variables|Character|GetMesh)) (Variables|Default|GetAttackRange) (Utilities|Array|MakeArray "ObjectTypeQuery3") "/Game/Blueprints/Actors/CombatCharacters/PC_Character.PC_Character_C" (Utilities|Array|MakeArray self)))
  (if _returnvalue
    (Class|LowEntryExtendedStandardLibrary|SortObjectArrayDirectly _outactors (EventDispatchers|CreateEvent :!event DistanceComparator) false)
    (bind _array_element (Utilities|Array|ForEachLoopwithBreak _outactors :!label _label)
      (:LoopBody
        (bind _aspc_character (Utilities|Casting|CastToPC_Character _array_element))
        (bind _isalive (Default|IsAlive _aspc_character))
        (if _isalive
          (bind _los (PCGeneral|HasLineOfSighttoTarget _aspc_character))
          (if _los
            (Variables|PCState|SetTarget _aspc_character)
            (goto _label Break))))
      (:Completed
        ;;[0 1 0.476 1 10] 2nd loop means no living line of sight enemies - ignore line of sight
        (Utilities|IsValid (Variables|PCState|GetTarget)
          (:Is%20Not%20Valid
            (bind _array_element_2 (Utilities|Array|ForEachLoopwithBreak _outactors :!label _label_2)
              (:LoopBody
                (bind _aspc_character_2 (Utilities|Casting|CastToPC_Character _array_element_2))
                (bind _isalive_2 (Default|IsAlive _aspc_character_2))
                (if _isalive_2
                  (Variables|PCState|SetTarget _aspc_character_2)
                  (goto _label_2 Break))))))))))

(event Custom|TryDreamBolt
  ;[0 1 0.476] TryDreamBolt: Should be stationary when called.
  ; Begin the autoattack. Animation notify will trigger subsequent attacks. Always try to shoot dream bolt if there's a valid target.
  (Utilities|IsValid (Variables|PCState|GetTarget)
    (:Is%20Valid
      (PCStateManagement|RotatetoTarget)
      (if (Variables|PCState|GethasStartedAttacking)
        ;;[0 1 0.476 1 10] Subsequent attacks come here
        (Variables|PCState|SethasNextAttack true)
        (else
          ;;[0 1 0.476 1 10] First attack comes here
          (Variables|PCState|SethasStartedAttacking true)
          (PCCombat|PlayAttackAnimMontage))))
    (:Is%20Not%20Valid
      (PCCombat|ResetAttackState))))

(event Custom|PlayDeathAnimThenDestroy
  ;[0 1 0.476] PlayDeathAnimThenDestroy: Choose a death animation to play, then destroy actor after anim finishes.
  (bind _deathanimmontage (PCGeneral|ChooseRandomDeathMontage))
  (bind _returnvalue (Animation|PlayAnimMontage _deathanimmontage 1.0 "None"))
  (Utilities|FlowControl|Delay _returnvalue)
  (Actor|DestroyActor))

(event Custom|HandleJump
  ;[0.9249 0.3262 1] Double jump logic
  (Utilities|IsAbilityEnabled "NewEnumerator3"
    (:Enabled
      (bind _counter (Utilities|FlowControl|DoN 2)
        (:Exit
          (switch int _counter
            (:1
              (Character|Jump :!label _label))
            (:2
              (Utilities|IsMpSufficient "NewEnumerator3"
                (:True
                  (Character|LaunchCharacter "0.000000,0.000000,420.000000" false false)
                  (PCAbilities|ReduceMP "NewEnumerator3")
                  (Variables|PCState|SetJustDoubleJumped true))))))))
    (:Disabled
      (goto _label))))

(event Custom|NextAttack
  ;[0 1 0.476] TryDreamBolt: Should be stationary when called.
  ; Begin the autoattack. Animation notify will trigger subsequent attacks. Always try to shoot dream bolt if there's a valid target.
  ;;[0 1 0.476 1 10] NextAttack: Triggered by end of attack anim in anim notify, unless attack state was reset by movement.
  (if (Variables|PCState|GethasNextAttack)
    (Variables|PCState|SethasNextAttack false)
    (Utilities|IsValid (Variables|PCState|GetTarget)
      (:Is%20Valid
        (PCCombat|PlayAttackAnimMontage))
      (:Is%20Not%20Valid
        (PCCombat|ResetAttackState)))))

(event EventBeginPlay
  (|CallParentFunction)
  ;[1 1 1] Set MP bar owner
  (PC_Construction|SetMPBarOwner))

(event Collision|EventActorBeginOverlap
  (params (OtherActor :type Actor%20Object%20Reference))
  (|CallParentFunction OtherActor) ; This node is disabled and will not be called.\nDrag off pins to build functionality.
)

(event EventTick
  (params (DeltaSeconds :type Float%20%28single-precision%29))
  (|CallParentFunction DeltaSeconds)
  ;[1 1 1] Only do things if HP > 0.
  (bind _isalive (CallFunction|IsAlive))
  (if _isalive
    ;[1 1 1] Update State
    (PCStateManagement|CheckifStationary)
    (PCCombat|IfMovingResetAttackState)
    ;[0 1 0.476] Enter combat if stationary and dream bolt enabled - try to autoattack.
    (Utilities|IsAbilityEnabled "NewEnumerator0"
      (:Enabled
        (if (Variables|PCState|GetisStationary)
          (PCCombat|TryGetNewTarget)
          (CallFunction|TryDreamBolt))))))

(event EventBlink
  ;[0.9249 0.3262 1] Perform Blink
  (PC_Abilities|ExecuteBlink))

(event EventOnLanded
  (params (Hit :type Hit%20Result%20Structure%20%28by%20ref%29))
  ;[0.9249 0.3262 1] Double jump logic
  (Utilities|FlowControl|DoN 2) ; enters at Reset
)

(fn ConstructionScript
  (|CallParentFunction))

(fn DistanceComparator
  (params (ObjectA :type Object%20Object%20Reference) (ObjectB :type Object%20Object%20Reference))
  (bind _mesh (Variables|Character|GetMesh))
  (bind _returnvalue (Transformation|GetWorldLocation _mesh))
  (bind _asactor (Utilities|Casting|CastToActor ObjectA))
  (bind _asactor_2 (Utilities|Casting|CastToActor ObjectB))
  (return (< (Math|Vector|Distance(Vector) (Transformation|GetActorLocation _asactor) _returnvalue) (Math|Vector|Distance(Vector) _returnvalue (Transformation|GetActorLocation _asactor_2)))))

(fn CheckifStationary
  (Variables|PCState|SetisStationary (== (Math|Vector|VectorLength (Pawn|Components|CharacterMovement|GetCurrentAcceleration (Variables|Character|GetCharacterMovement))) 0.0)))

(fn IfMovingResetAttackState
  (if (not (Variables|PCState|GetisStationary))
    (PCCombat|ResetAttackState)))

(fn RotatetoTarget
  (Transformation|SetWorldRotation (Variables|Default|GetCapsuleComponent) (Math|Interpolation|RInterpTo (Math|Rotator|MakeRotator 0.0 0.0 (.yaw (Transformation|GetWorldRotation (Variables|Default|GetCapsuleComponent)))) (Math|Rotator|MakeRotator 0.0 0.0 (.yaw (Math|Rotator|FindLookatRotation (Transformation|GetWorldLocation (Variables|Default|GetCapsuleComponent)) (Transformation|GetWorldLocation (Variables|/Script/Engine.Character|GetMesh (Variables|PCState|GetTarget)))))) (Variables|Default|GetDeltaSeconds) 15.0) false false))

(fn PlayAttackAnimMontage
  (bind _attackrate (Variables|PCStats|GetAttackRate))
  (switch int (Variables|PCState|GetAttackCount)
    (:0
      (Variables|PCState|SetAttackCount 1)
      (Animation|PlayAnimMontage "/Game/Assets/Characters/ElinaSomnia/Animations/AM_AutoAttackA.AM_AutoAttackA" _attackrate "None"))
    (:1
      (Variables|PCState|SetAttackCount 2)
      (Animation|PlayAnimMontage "/Game/Assets/Characters/ElinaSomnia/Animations/AM_AutoAttackB.AM_AutoAttackB" _attackrate "None"))
    (:2
      (Variables|PCState|SetAttackCount 3)
      (Animation|PlayAnimMontage "/Game/Assets/Characters/ElinaSomnia/Animations/AM_AutoAttackC.AM_AutoAttackC" _attackrate "None"))
    (:3
      (Variables|PCState|SetAttackCount 0)
      (Animation|PlayAnimMontage "/Game/Assets/Characters/ElinaSomnia/Animations/AM_AutoAttackD.AM_AutoAttackD" _attackrate "None"))))

(fn ResetAttackState
  (Variables|PCState|SethasStartedAttacking false)
  (Variables|PCState|SetAttackCount 0)
  (Variables|PCState|SethasNextAttack false)
  (Variables|PCState|SetTarget 0)
  (Animation|StopAnimMontage 0))

(fn SpawnDreamBoltTowardTarget
  (bind _dreamboltspawnpoint (Variables|PC_Temp|GetDreamBoltSpawnPoint))
  (Game|SpawnActorfromClass "/Game/Blueprints/Actors/Combat/Projectiles/BP_DreamBolt.BP_DreamBolt_C" (Math|Transform|MakeTransform _dreamboltspawnpoint (Math|Rotator|FindLookatRotation _dreamboltspawnpoint (Transformation|GetWorldLocation (Variables|/Script/Engine.Actor|GetRootComponent (Variables|PCState|GetTarget)))) "1,1,1") "Undefined" 0 (Variables|PCStats|GetDreamBoltDmg) self))

(fn KillCharacter
  (CallFunction|PlayDeathAnimThenDestroy))

(fn ChooseRandomDeathMontage
  (switch int (Math|Random|RandomIntegerinRange 0 2)
    (:0
      (LocalVariables|SetSelectedAnimMontage "/Game/Assets/Characters/ElinaSomnia/Animations/AM_Death1.AM_Death1"))
    (:1
      (LocalVariables|SetSelectedAnimMontage "/Game/Assets/Characters/ElinaSomnia/Animations/AM_Death2.AM_Death2"))
    (:2
      (LocalVariables|SetSelectedAnimMontage "/Game/Assets/Characters/ElinaSomnia/Animations/AM_Death3.AM_Death3")))
  (return (LocalVariables|GetSelectedAnimMontage)))

(fn HasLineOfSighttoTarget
  (params (TargetCandidate :type PC%20Character%20Object%20Reference))
  (bind _returnvalue (Collision|SphereTraceByChannel (Transformation|GetWorldLocation (Variables|Default|GetCapsuleComponent)) (Transformation|GetWorldLocation (Variables|/Script/Engine.Actor|GetRootComponent TargetCandidate)) 8.0 "TraceTypeQuery1" false (Utilities|Array|MakeArray TargetCandidate self) "ForDuration" true "(R=1.000000,G=0.000000,B=0.000000,A=1.000000)" "(R=0.000000,G=1.000000,B=0.000000,A=1.000000)" 1.0))
  (return (not _returnvalue)))

(fn FireDreamBolt
  (params (AttackingHand :type LRHand%20Enum :default "NewEnumerator0"))
  ;[0 1 0.476] FireDreamBolt: Make sure target is valid, rotate to target, set the spawning hand location then spawn bolt toward target. Called by anim notify.
  (Utilities|IsValid (Variables|PCState|GetTarget)
    (:Is%20Valid
      (PCStateManagement|RotatetoTarget)
      ;;[0 1 0.476 1 10] Get spawn point and rotation to target.
      (switch Utilities|FlowControl|Switch|SwitchonLRHand AttackingHand
        (:NewEnumerator0
          (Variables|PC_Temp|SetDreamBoltSpawnPoint (Transformation|GetSocketLocation (Variables|Character|GetMesh) "hand_l")))
        (:NewEnumerator1
          (Variables|PC_Temp|SetDreamBoltSpawnPoint (Transformation|GetSocketLocation (Variables|Character|GetMesh) "hand_r"))))
      (PC_Combat|SpawnDreamBoltTowardTarget))
    (:Is%20Not%20Valid
      (PCCombat|ResetAttackState))))

(fn TryGetNewTarget
  (bind _target (Variables|PCState|GetTarget))
  ;[0 1 0.476] TryGetNewTarget: Should be stationary when called.
  ; If player doesn't have a valid/alive target (just became stationary or target just died), get new target.
  (Utilities|IsValid _target
    (:Is%20Valid
      (bind _isalive (Default|IsAlive _target))
      (if (not _isalive)
        (CallFunction|FindClosestTarget :!label _label)))
    (:Is%20Not%20Valid
      (goto _label))))

(fn ExecuteBlink
  (bind _capsulecomponent (Variables|Default|GetCapsuleComponent))
  (bind _blinkrange (Variables|PCAttributes|GetBlinkRange))
  (bind _capsulecomponent_2 (Variables|Default|GetCapsuleComponent))
  (bind _returnvalue (Transformation|GetWorldLocation _capsulecomponent))
  (bind _returnvalue_2 (Transformation|GetWorldRotation _capsulecomponent_2))
  (bind _returnvalue_3 (Math|Vector|GetForwardVector _returnvalue_2))
  (bind _returnvalue_4 (* _returnvalue_3 _blinkrange))
  (Utilities|IsAbilityEnabled "NewEnumerator1"
    (:Enabled
      (Utilities|IsMpSufficient "NewEnumerator1"
        (:True
          (bind _aspc_game_state (Utilities|Casting|CastToPC_GameState (Game|GetGameState))
            (:then
              (bind (_outhit _returnvalue_5) (Collision|LineTraceForObjects _returnvalue (+ _returnvalue _returnvalue_4) (Utilities|Array|MakeArray "ObjectTypeQuery1") false (Variables|/Game/Blueprints/GameLogic/PC_GameState.PC_GameState_C|GetBlinkableObjects _aspc_game_state) "ForDuration" true "(R=1.000000,G=0.000000,B=0.000000,A=1.000000)" "(R=0.000000,G=1.000000,B=0.000000,A=1.000000)" 1.0))
              (Effects|SpawnEmitteratLocation "/Game/Assets/Effects/Blink/PE_Blink.PE_Blink" (Transformation|GetWorldLocation (Variables|Character|GetMesh)) "0, 0, 0" "0.100000,0.100000,0.100000")
              (if _returnvalue_5
                ;[1 1 1] If there's something blocking, blink up to that blocking body.
                (Transformation|Teleport (.Location (Collision|BreakHitResult _outhit)) (Transformation|GetWorldRotation (Variables|Default|GetCapsuleComponent)))
                (Effects|SpawnEmitteratLocation "/Game/Assets/Effects/Blink/PE_Blink.PE_Blink" (Transformation|GetWorldLocation (Variables|Character|GetMesh)) "0, 0, 0" "0.100000,0.100000,0.100000")
                (else
                  ;[1 1 1] If there's nothing blocking, just blink forward with blink direction vector.
                  (Transformation|AddWorldOffset (Variables|Default|GetCapsuleComponent) _returnvalue_4 false true)
                  (Effects|SpawnEmitteratLocation "/Game/Assets/Effects/Blink/PE_Blink.PE_Blink" (Transformation|GetWorldLocation (Variables|Character|GetMesh)) "0, 0, 0" "0.100000,0.100000,0.100000")))
              (PCAbilities|ReduceMP "NewEnumerator1"))
            (:CastFailed
              (Development|PrintString "Use PC_GameState to allow blinking."))))
        (:False
          (Development|PrintString "Insufficient MP to blink."))))
    (:Disabled
      (Development|PrintString "Blink is not enabled in game instance."))))

(fn ReduceMP
  (params (Ability :type PC_Abilities%20Enum :default "NewEnumerator0"))
  (bind _aspc_game_instance (Utilities|Casting|CastToPC_GameInstance (Game|GetGameInstance)))
  (switch Utilities|FlowControl|Switch|SwitchonPC_Abilities Ability
    (:NewEnumerator1
      (LocalVariables|SetCost (Variables|/Game/Blueprints/GameLogic/PC_GameInstance.PC_GameInstance_C|GetcostBlink _aspc_game_instance)))
    (:NewEnumerator2
      (LocalVariables|SetCost (Variables|/Game/Blueprints/GameLogic/PC_GameInstance.PC_GameInstance_C|GetcostDreamBarrage _aspc_game_instance)))
    (:NewEnumerator3
      (LocalVariables|SetCost (Variables|/Game/Blueprints/GameLogic/PC_GameInstance.PC_GameInstance_C|GetcostDoubleJump _aspc_game_instance)))
    (:NewEnumerator4
      (LocalVariables|SetCost (Variables|/Game/Blueprints/GameLogic/PC_GameInstance.PC_GameInstance_C|GetcostConfusion _aspc_game_instance)))
    (:NewEnumerator5
      (LocalVariables|SetCost (Variables|/Game/Blueprints/GameLogic/PC_GameInstance.PC_GameInstance_C|GetcostIsolation _aspc_game_instance)))
    (:NewEnumerator6
      (LocalVariables|SetCost (Variables|/Game/Blueprints/GameLogic/PC_GameInstance.PC_GameInstance_C|GetcostParalyze _aspc_game_instance)))
    (:NewEnumerator7
      (LocalVariables|SetCost (Variables|/Game/Blueprints/GameLogic/PC_GameInstance.PC_GameInstance_C|GetcostTimeFreeze _aspc_game_instance)))
    (:NewEnumerator8
      (LocalVariables|SetCost (Variables|/Game/Blueprints/GameLogic/PC_GameInstance.PC_GameInstance_C|GetcostMaim _aspc_game_instance))))
  (Variables|Default|SetMP (- (Variables|Default|GetMP) (LocalVariables|GetCost))))

(fn SetMPBarOwner
  (bind _aspc_mpbar (Utilities|Casting|CastToPC_MPBar (UserInterface|GetUserWidgetObject (Variables|Default|GetMPBar))))
  (Default|SetOwningCharacter _aspc_mpbar self))