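; Miseria is an AI combat character with a three-hit dream bolt combo, radial Dream Barrage, Dream Rifts around its target and minion summoning.
; Behavior tree tasks trigger attacks, which turn briefly, then play montages if Miseria is alive and no dialog is playing.
; Parent-class overrides spawn projectiles and enemy spawners, while laser prediction lines telegraph bolts and barrage.
; Summoning requires at most one enemy left in PC_GameState.
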(event Custom|PlayDeathAnimThenDestroy
  ;[1 1 1] Choose a random death anim montage to play then destroy the actor
  (bind _deathanimmontage (CallFunction|ChooseRandomDeathMontage))
  (bind _returnvalue (Animation|PlayAnimMontage _deathanimmontage 1.0 "None"))
  (Utilities|FlowControl|Delay _returnvalue)
  (Actor|DestroyActor))

(event Custom|SpawnRadialPred
  (bind _dreambarragenum (Variables|PCAbilities|GetDreamBarrageNum))
  (bind _capsulecomponent (Variables|Default|GetCapsuleComponent))
  (bind _returnvalue (Transformation|GetWorldRotation _capsulecomponent))
  ;[1 1 1] Spawn radial prediction lines in even intervals in a circle around the player, leaving 0.5s before the fire event.
  (Variables|PCTemp|SetDreamBarragePLInterval (/ (- (Variables|PCAbilities|GetDreamBarrageTelegraph) 0.5) (Math|Conversions|ToFloat(Integer) (Variables|PCAbilities|GetDreamBarrageNum))))
  (if (<= (Variables|PCTemp|GetDreamBarrageIdx) _dreambarragenum) :!label _label
    (bind _returnvalue_2 (Game|SpawnActorfromClass "/Game/Blueprints/Actors/Combat/PredictionLines/BP_LaserPredictionLines.BP_LaserPredictionLines_C" (Math|Transform|MakeTransform (+ (* (Math|Vector|GetForwardVector (Math|Rotator|MakeRotator 0.0 0.0 (+ (.yaw _returnvalue) (* (Variables|PCTemp|GetDreamBarrageIdx) (/ 3.6e+02 (Math|Conversions|ToFloat(Integer) _dreambarragenum)))))) 1e+02) (Transformation|GetWorldLocation (Variables|Default|GetCapsuleComponent))) (Math|Rotator|MakeRotator (.roll _returnvalue) (.pitch _returnvalue) (+ (.yaw _returnvalue) (* (Variables|PCTemp|GetDreamBarrageIdx) (/ 3.6e+02 (Math|Conversions|ToFloat(Integer) _dreambarragenum))))) "1,1,1") "Undefined" 0 self))
    (Utilities|Array|Add (Variables|PC_Temp|GetLaserRef) _returnvalue_2)
    (Math|Integer|IncrementInt (Variables|PCTemp|GetDreamBarrageIdx)
      (:%20%20
        (Utilities|FlowControl|Delay (Variables|PCTemp|GetDreamBarragePLInterval))
        (goto _label)))
    (else
      (Variables|PCTemp|SetDreamBarrageIdx 1))))

(event EventBeginPlay
  (|CallParentFunction) ; This node is disabled and will not be called.\nDrag off pins to build functionality.
)

(event Collision|EventActorBeginOverlap
  (params (OtherActor :type Actor%20Object%20Reference))
  (|CallParentFunction OtherActor) ; This node is disabled and will not be called.\nDrag off pins to build functionality.
)

(event EventTick
  (params (DeltaSeconds :type Float%20%28single-precision%29))
  (|CallParentFunction DeltaSeconds) ; This node is disabled and will not be called.\nDrag off pins to build functionality.
)

(event EventTryPrimaryAttack
  ;[1 1 1] Called by the behavior tree task PC_PrimaryAttack. This will end up calling notifies for NextAttack.
  (PCCombat|SpawnFrontPL)
  (Utilities|RotateforDuration 0.5
    (:Out
      (PCCombat|DeleteAllPLs)
      (Utilities|IsActionAllowed
        (:T
          (bind _chosenanimmontage (PC_Combat|GetAutoattackAnim (Variables|PCState|GetAttackNumber)))
          (Animation|PlayAnimMontage _chosenanimmontage 1.0 "None"))))))

(event EventTryDreamBarrage
  ;[1 1 1] Called by FireDreamBarrage PC_AnimTrigger, which is called by behavior tree task PC_DreamBarrage.
  (Utilities|RotateforDuration 0.5
    (:Out
      (Utilities|IsActionAllowed
        (:T
          (Animation|PlayAnimMontage "/Game/Assets/Characters/Common/ES_Animations/AM_ES_M_DreamBarrage.AM_ES_M_DreamBarrage" 1.0 "None")
          (CallFunction|SpawnRadialPred)
          (Utilities|FlowControl|Delay (Variables|PCAbilities|GetDreamBarrageTelegraph))
          (PCCombat|DeleteAllPLs))))))

(event EventTryDreamRift
  ;[1 1 1] Called by PC_DreamRift
  (Utilities|RotateforDuration 0.5
    (:Out
      (Utilities|IsActionAllowed
        (:T
          (Animation|PlayAnimMontage "/Game/Assets/Characters/Common/ES_Animations/AM_ES_M_CosmicRift_Start.AM_ES_M_CosmicRift_Start" 1.0 "None")
          (PCCombat|SpawnDreamRifts))))))

(event EventTrySummonMinionsEvent
  ;[1 1 1] Called by PC_SummonMinion
  (Utilities|RotateforDuration 0.5
    (:Out
      (Utilities|IsActionAllowed
        (:T
          (Animation|PlayAnimMontage "/Game/Assets/Characters/Common/ES_Animations/AM_ES_M_Ability_E.AM_ES_M_Ability_E" 1.0 "None"))))))

(fn ConstructionScript
  (|CallParentFunction))

(fn ChooseRandomDeathMontage
  (switch int (Math|Random|RandomIntegerinRange 0 3)
    (:0
      (LocalVariables|SetSelectedAnimMontage "/Game/Assets/Characters/Common/ES_Animations/AM_ES_Death1.AM_ES_Death1"))
    (:1
      (LocalVariables|SetSelectedAnimMontage "/Game/Assets/Characters/Common/ES_Animations/AM_ES_Death2.AM_ES_Death2"))
    (:2
      (LocalVariables|SetSelectedAnimMontage "/Game/Assets/Characters/Common/ES_Animations/AM_ES_Death3.AM_ES_Death3"))
    (:3
      (LocalVariables|SetSelectedAnimMontage "/Game/Assets/Characters/Common/ES_Animations/AM_ES_Death_Fwd_Montage.AM_ES_Death_Fwd_Montage")))
  (return (LocalVariables|GetSelectedAnimMontage)))

(fn KillCharacter
  (CallFunction|DisableCollisions)
  (CallFunction|PlayDeathAnimThenDestroy)
  (CallFunction|NotifyDeathtoGameState))

(fn FireAutoattack
  (params (AttackingHand :type LRHand%20Enum :default "NewEnumerator0"))
  (bind _mesh (Variables|Character|GetMesh))
  (|CallParentFunction AttackingHand)
  (switch Utilities|FlowControl|Switch|SwitchonLRHand AttackingHand
    (:NewEnumerator0
      (PCCombat|SpawnDreamBoltTowardTarget (Transformation|GetSocketLocation _mesh "hand_l")))
    (:NewEnumerator1
      (PCCombat|SpawnDreamBoltTowardTarget (Transformation|GetSocketLocation _mesh "hand_r")))))

(fn GetAutoattackAnim
  (params (AttackNo :type Integer))
  (switch int AttackNo
    (:Default
      (LocalVariables|SetAnimMontage "/Game/Assets/Characters/Common/ES_Animations/AM_M_Primary_Attack_A_Medium.AM_M_Primary_Attack_A_Medium" :!label _label))
    (:0
      (goto _label))
    (:1
      (LocalVariables|SetAnimMontage "/Game/Assets/Characters/Common/ES_Animations/AM_M_Primary_Attack_B_Medium.AM_M_Primary_Attack_B_Medium"))
    (:2
      (LocalVariables|SetAnimMontage "/Game/Assets/Characters/Common/ES_Animations/AM_M_Primary_Attack_C_Medium.AM_M_Primary_Attack_C_Medium")))
  (return (LocalVariables|GetAnimMontage)))

(fn NextAttack
  (|CallParentFunction)
  (bind _result (Math|Integer|IncrementInt (Variables|PCState|GetAttackNumber))
    (:%20%20
      (if (< _result 3)
        ;[1 1 1] If it's still valid attack number, play the next attack.
        (bind _chosenanimmontage (PC_Combat|GetAutoattackAnim _result))
        (Animation|PlayAnimMontage _chosenanimmontage 1.0 "None")
        (else
          ;[1 1 1] Otherwise reset for next set of attacks.
          (Variables|PCState|SetAttackNumber 0))))))

(fn FireDreamBarrage
  (bind _capsulecomponent (Variables|Default|GetCapsuleComponent))
  (bind _dreambarragenum (Variables|PCAbilities|GetDreamBarrageNum))
  (bind _returnvalue (Transformation|GetWorldRotation _capsulecomponent))
  (|CallParentFunction)
  (for _index (range 1 _dreambarragenum)
    (Game|SpawnActorfromClass "/Game/Blueprints/Actors/Combat/Projectiles/PC_BP_DreamBarrage.PC_BP_DreamBarrage_C" (Math|Transform|MakeTransform (+ (Transformation|GetWorldLocation (Variables|Default|GetCapsuleComponent)) (* (Math|Vector|GetForwardVector (Math|Rotator|MakeRotator 0.0 0.0 (+ (.yaw _returnvalue) (* _index (/ 3.6e+02 (Math|Conversions|ToFloat(Integer) _dreambarragenum)))))) 1e+02)) (Math|Rotator|MakeRotator (.roll _returnvalue) (.pitch _returnvalue) (+ (.yaw _returnvalue) (* _index (/ 3.6e+02 (Math|Conversions|ToFloat(Integer) _dreambarragenum))))) "3.000000,3.000000,3.000000") "Undefined" 0 (* (Variables|PC_Abilities|GetDreamBarrageMultiplier) (Variables|Default|GetPrimaryAttackDmg)) 8e+02 self)))

(fn SpawnDreamBoltTowardTarget
  (params (SpawnPoint :type Vector))
  (Game|SpawnActorfromClass "/Game/Blueprints/Actors/Combat/Projectiles/PC_BP_DreamBolt.PC_BP_DreamBolt_C" (Math|Transform|MakeTransform SpawnPoint (Transformation|GetWorldRotation (Variables|Default|GetCapsuleComponent)) "3.000000,3.000000,3.000000") "Undefined" 0 (Variables|Default|GetPrimaryAttackDmg) 1e+03 0))

(fn SpawnFrontPL
  (bind _capsulecomponent (Variables|Default|GetCapsuleComponent))
  (bind _returnvalue (Transformation|GetWorldTransform _capsulecomponent))
  (bind _returnvalue_2 (Game|SpawnActorfromClass "/Game/Blueprints/Actors/Combat/PredictionLines/BP_LaserPredictionLines.BP_LaserPredictionLines_C" (Math|Transform|MakeTransform (.location _returnvalue) (.rotation _returnvalue) "1,1,1") "Undefined" 0 0))
  (Utilities|Array|Add (Variables|PC_Temp|GetLaserRef) _returnvalue_2))

(fn DeleteAllPLs
  (bind _laserref (Variables|PC_Temp|GetLaserRef))
  (for _array_element _laserref
    (Actor|DestroyActor _array_element))
  (Utilities|Array|Clear _laserref))

(fn RotatetoTarget
  (params (TargetEnemy :type PC%20BP%20Character%20Object%20Reference))
  (|CallParentFunction TargetEnemy)
  (for _array_element (Variables|PC_Temp|GetLaserRef)
    (Transformation|SetWorldRotation (Variables|/Game/Blueprints/Actors/Combat/PredictionLines/BP_LaserPredictionLines.BP_LaserPredictionLines_C|GetDefaultSceneRoot _array_element) (.rotation (Transformation|GetWorldTransform (Variables|Default|GetCapsuleComponent))) false false)))

(fn SpawnDreamRifts
  (bind _targetenemy (Variables|Default|GetTargetEnemy))
  (bind _mesh (Variables|Character|GetMesh))
  (bind _returnvalue (Transformation|GetWorldLocation _mesh))
  (bind _capsulecomponent (Variables|/Script/Engine.Character|GetCapsuleComponent _targetenemy))
  (bind _returnvalue_2 (Transformation|GetWorldLocation _capsulecomponent))
  (bind _returnvalue_3 (+ (.z _returnvalue) 1.0))
  (bind _returnvalue_4 (Math|Vector|MakeVector (.x _returnvalue_2) (.y _returnvalue_2) _returnvalue_3))
  (Game|SpawnActorfromClass "/Game/Blueprints/Actors/Combat/Projectiles/PC_BP_DreamRift.PC_BP_DreamRift_C" (Math|Transform|MakeTransform _returnvalue_4 "0, 0, 0" "1,1,1") "Undefined" 0 (Variables|PCAbilities|GetDreamRiftRadius) (Variables|PCAbilities|GetDreamRiftTelegraph) 3e+01 0)
  (bind _locations (PCCombat|GetRiftLocations _returnvalue_4))
  (for _array_element _locations
    (Game|SpawnActorfromClass "/Game/Blueprints/Actors/Combat/Projectiles/PC_BP_DreamRift.PC_BP_DreamRift_C" (Math|Transform|MakeTransform _array_element "0, 0, 0" "1,1,1") "Undefined" 0 (Variables|PCAbilities|GetDreamRiftRadius) (Variables|PCAbilities|GetDreamRiftTelegraph) (* (Variables|Default|GetPrimaryAttackDmg) (Variables|PCAbilities|GetDreamRiftMultiplier)) self)))

(fn GetRiftLocations
  (params (StartLocation :type Vector))
  (bind _dreamriftradius (Variables|PCAbilities|GetDreamRiftRadius))
  (bind _returnvalue (* _dreamriftradius 2.0))
  (bind _randomlocation (Class|NavigationSystemV1|GetRandomPointinNavigableRadius StartLocation _returnvalue 0 0))
  (for _index (range 1 (Variables|PCAbilities|GetDreamRiftNum))
    (Utilities|Array|Add (LocalVariables|GetResult) (Math|Vector|MakeVector (.x _randomlocation) (.y _randomlocation) (+ (.z (Transformation|GetWorldLocation (Variables|Character|GetMesh))) 1.0))))
  (return (LocalVariables|GetResult)))

(fn TrySummonMinions
  (bind _aspc_game_state (Utilities|Casting|CastToPC_GameState (Game|GetGameState))
    (:then
      (if (<= (Variables|/Game/Blueprints/GameLogic/PC_GameState.PC_GameState_C|GetEnemiesLeft _aspc_game_state) 1)
        (Utilities|IsActionAllowed
          (:T
            (CallFunction|TrySummonMinionsEvent)
            (return true))
          (:F
            _)))
      (return false))
    (:CastFailed
      (Development|PrintString "PC_BP_Miseria::TrySummonMinions: Use PC Gamestate!"))))

(fn SpawnChars
  (|CallParentFunction)
  (Utilities|IsActionAllowed
    (:T
      (for _array_element (Variables|PCAbilities|GetSpawnEnemiesStruct)
        (for _index (range 1 (.number _array_element))
          (Game|SpawnActorfromClass "/Game/Blueprints/Actors/Combat/Spawners/PC_BP_EnemySpawner.PC_BP_EnemySpawner_C" (Math|Transform|MakeTransform (.RandomLocation (Class|NavigationSystemV1|GetRandomPointinNavigableRadius (Transformation|GetWorldLocation (Variables|Default|GetCapsuleComponent)) (Variables|PCAbilities|GetSpawnEnemiesRadius) 0 0)) "0, 0, 0" "1,1,1") "Undefined" 0 (.enemytype _array_element) (.aggrorange _array_element) (.primaryattackdmg _array_element) (.maxhp _array_element) self)
          (bind _aspc_game_state (Utilities|Casting|CastToPC_GameState (Game|GetGameState)))
          (Default|AddEnemy _aspc_game_state))))))