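; Combat character Blueprint that manages health, mana, damage and death.
; BeginPlay applies the walk speed and registers the character with its HP bar widget.
; While alive, Tick regenerates MP continuously and HP only after a delay since the last hit, both clamped to their maximums.
; Damage lowers HP and records the hit time; reaching zero destroys the actor, guarded by a DoOnce.
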(event EventBeginPlay
  ;[1 1 1] Set movement component max walk speed
  (PCConstruction|SetMaxWalkSpeed)
  ;[1 1 1] Set HP bar owner
  (PCConstruction|SetHPBarOwner))

(event Game|Damage|EventAnyDamage
  (params (Damage :type Float%20%28single-precision%29) (DamageType :type Damage%20Type%20Object%20Reference) (InstigatedBy :type Controller%20Object%20Reference) (DamageCauser :type Actor%20Object%20Reference))
  ;[1 1 1] Reduce health
  (PCStateManagement|ReduceHealth Damage)
  ;[1 1 1] Trigger death sequence if dead.
  (bind _isalive (PC_StateManagement|IsAlive))
  (if (not _isalive)
    (Utilities|FlowControl|DoOnce false
      (:Completed
        (PC_Overridable|KillCharacter)))))

(event EventTick
  (params (DeltaSeconds :type Float%20%28single-precision%29))
  (Variables|PC_References|SetDeltaSeconds DeltaSeconds)
  ;[1 1 1] Only do things if HP > 0.
  (bind _isalive (PC_StateManagement|IsAlive))
  (if _isalive
    ;[1 1 1] Regen HP/MP
    (PC_StateManagement|Regen)))

(fn ConstructionScript)

(fn SetMaxWalkSpeed
  (Variables|/Script/Engine.CharacterMovementComponent|SetMaxWalkSpeed (Variables|Character|GetCharacterMovement) (Variables|PC_Attributes|GetWalkSpeed)))

(fn IsAlive
  (return (> (Variables|PC_State|GetHP) 0.0)))

(fn Regen
  ;[1 1 1] Regen HP only if sufficient time since last damaged passed.
  (if (> (- (Utilities|Time|GetTimeSeconds) (Variables|PCReferences|GetTimeDamaged)) (Variables|PCStats|GetTimeBeforeHPRegen))
    ;[1 1 1] Regen HP
    (Variables|PC_State|SetHP (Math|Float|Clamp(Float) (+ (Variables|PC_State|GetHP) (* (Variables|PC_Stats|GetHPRegen) (Variables|PC_References|GetDeltaSeconds))) 0.0 (Variables|PC_Stats|GetMaxHP))))
  ;[1 1 1] Regen MP
  (Variables|PC_State|SetMP (Math|Float|Clamp(Float) (+ (Variables|PC_State|GetMP) (* (Variables|PC_Stats|GetMPRegen) (Variables|PC_References|GetDeltaSeconds))) 0.0 (Variables|PC_Stats|GetMaxMP))))

(fn ResetHPMP
  (Variables|PC_State|SetHP (Variables|PC_Stats|GetMaxHP))
  (Variables|PC_State|SetMP (Variables|PC_Stats|GetMaxMP)))

(fn ReduceHealth
  (params (Damage :type Float%20%28single-precision%29))
  (Variables|PC_State|SetHP (Math|Float|Max(Float) 0.0 (- (Variables|PC_State|GetHP) Damage)))
  (Variables|PCReferences|SetTimeDamaged (Utilities|Time|GetTimeSeconds))
  (return))

(fn KillCharacter
  (Actor|DestroyActor))

(fn SetHPBarOwner
  (bind _aspc_health_bar (Utilities|Casting|CastToPC_HealthBar (UserInterface|GetUserWidgetObject (Variables|Default|GetHPBar))))
  (Default|SetOwningCharacter _aspc_health_bar self))