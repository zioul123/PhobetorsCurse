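; PC_NPCBase is a base NPC that hands its dialogue tree to its AI controller and starts dialogue on interaction.
; On BeginPlay it copies its DialogueTree into the PC_AIC_NPCBase controller.
; Its Interact event casts to that controller and calls StartDialogue, so the controller handles the conversation itself.
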(event Custom|SetAICDialogueTree
  ;[1 1 1] Set dialogue tree of AI controller to the dialogue tree given to this NPC base
  (bind _aspc_aic_npcbase (Utilities|Casting|CastToPC_AIC_NPCBase (AI|GetAIController self)))
  (Variables|/Game/Blueprints/Controllers/AI_NPCs/PC_AIC_NPCBase.PC_AIC_NPCBase_C|SetDialogueTree _aspc_aic_npcbase (Variables|Default|GetDialogueTree)))

(event EventBeginPlay
  (CallFunction|SetAICDialogueTree))

(event EventInteract
  ;[1 1 1] Call controller's StartDialogue
  (bind _aspc_aic_npcbase (Utilities|Casting|CastToPC_AIC_NPCBase (AI|GetAIController self)))
  (Default|StartDialogue _aspc_aic_npcbase))

(fn ConstructionScript)