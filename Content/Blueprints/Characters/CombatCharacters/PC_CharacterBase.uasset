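; Base combat character with melee, magic projectiles, a Blink teleport, health and interaction detection.
; BeginPlay caches the HUD, links the health bar and attaches a spawned weapon to its socket.
; Melee combos chain through montage sections; damage reduces health, triggering timed flinches that block attacks, or a death montage before destroying character and weapon.
; Each tick, a forward sphere trace finds interactable-interface actors and toggles the HUD prompt.
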(event Custom|TryMelee
  (bind _mesh (Variables|Character|GetMesh))
  (bind _returnvalue (Components|SkeletalMesh|GetAnimInstance _mesh))
  (bind _returnvalue_2 (Animation|Montage|MontageGetCurrentSection _returnvalue "/Game/Assets/Knight/AM_KG_Melee.AM_KG_Melee"))
  ;[1 1 1 1 30] Combat
  ;;[1 1 1] TryMelee: If not currently flinching, if not currently attacking, play melee attack animation montage, otherwise set next anim section
  (if (not (Variables|Default|GetIsFlinching))
    (if (Animation|Montage|MontageIsPlaying _returnvalue "/Game/Assets/Knight/AM_KG_Melee.AM_KG_Melee")
      (switch name _returnvalue_2
        (:Attack1
          (Class|AnimInstance|MontageSetNextSection _returnvalue _returnvalue_2 "Attack2" 0)))
      (else
        (Animation|PlayAnimMontage "/Game/Assets/Knight/AM_KG_Melee.AM_KG_Melee" 1.0 "Attack1")))))

(event Custom|TryMagic
  ;[1 1 1 1 30] Combat
  ;;[1 1 1] TryMagic: If not flinching, play magic montage
  (if (not (Variables|Default|GetIsFlinching))
    (Animation|PlayAnimMontage "/Game/Assets/Knight/AM_KG_Magic.AM_KG_Magic" 1.0 "Default")))

(event Custom|CreateWeapon
  ;[1 1 1 1 30] Creation
  ;;[1 1 1] Create a weapon mesh and attach it to the weapon socket
  (bind _returnvalue (Game|SpawnActorfromClass (Variables|Default|GetWeaponClass) (Transformation|GetActorTransform) "Undefined" 0 0))
  (bind _output_get (Variables|Default|SetWeapon _returnvalue))
  (Transformation|AttachComponentToComponent _output_get (Variables|Character|GetMesh) "Weapon" "SnapToTarget" "SnapToTarget" "SnapToTarget" false))

(event Custom|KillCharacter
  ;[1 1 1 1 30] Damage and Death
  ;;[1 1 1] KillCharacter: Set flinch, play death animation and destroy actor and health bar
  (Variables|Default|SetIsFlinching true)
  (Pawn|Components|CharacterMovement|DisableMovement (Variables|Character|GetCharacterMovement))
  (bind _returnvalue (Animation|PlayAnimMontage "/Game/Assets/Knight/AM_KG_Death.AM_KG_Death" 1.0 "None"))
  (Utilities|FlowControl|Delay _returnvalue)
  (Actor|DestroyActor (Variables|Default|GetWeapon))
  (Actor|DestroyActor))

(event Custom|Flinch
  (bind _mesh (Variables|Character|GetMesh))
  (bind _returnvalue (Components|SkeletalMesh|GetAnimInstance _mesh))
  ;[1 1 1 1 30] Damage and Death
  ;;[1 1 1] Flinch: If not in midst of attack animation, set flinch, play flinch animation - if ending attack, big flinch, otherwise small flinch.
  (Variables|Default|SetIsFlinching true)
  (if (Animation|Montage|MontageIsPlaying _returnvalue "/Game/Assets/Knight/AM_KG_Melee.AM_KG_Melee")
    (if (Utilities|Array|ContainsItem (Variables|Default|GetAttackMoves) (Animation|Montage|MontageGetCurrentSection _returnvalue "/Game/Assets/Knight/AM_KG_Melee.AM_KG_Melee"))
      _
      (else
        (bind _returnvalue_2 (Animation|PlayAnimMontage "/Game/Assets/Knight/AM_KG_Flinch.AM_KG_Flinch" 1.0 "FlinchBig"))
        (Utilities|FlowControl|Delay _returnvalue_2)))
    (else
      (bind _returnvalue_3 (Animation|PlayAnimMontage "/Game/Assets/Knight/AM_KG_Flinch.AM_KG_Flinch" 1.0 "FlinchSmall"))
      (Utilities|FlowControl|Delay _returnvalue_3)))
  (Variables|Default|SetIsFlinching false))

(event Custom|LaunchMagicProjectile
  ;[1 1 1 1 30] Combat
  ;;[1 1 1] LaunchMagicProjectile: Spawn a magic projectile
  (Game|SpawnActorfromClass "/Game/Blueprints/Weapons/PC_ProjectileBase.PC_ProjectileBase_C" (Transformation|GetWorldTransform (Variables|Default|GetMagicSpawnPoint)) "Undefined" 0 self))

(event Custom|Blink
  ;[1 1 1] Innate Powers
  ;;[1 1 1] Blink: Spawn particles, teleport in that direction, and spawn more particles
  (Effects|SpawnEmitteratLocation "/Game/Assets/Effects/P_Blink.P_Blink" (Transformation|GetActorLocation))
  (Transformation|AddActorWorldOffset (* (Math|Vector|GetForwardVector (Transformation|GetActorRotation)) (Variables|Default|GetPowerRange)) false true)
  (Effects|SpawnEmitteratLocation "/Game/Assets/Effects/P_Blink.P_Blink" (Transformation|GetActorLocation)))

(event Custom|TryPrimaryAttack
  ;[1 1 1 1 30] Combat
  ;;[1 1 1] Use the primary attack - melee for base character
  (CallFunction|TryMelee))

(event Custom|GetHUD
  ;[1 1 1 1 30] Creation
  ;;[1 1 1] Get HUD reference
  (bind _aspc_game_mode_orig (Utilities|Casting|CastToPC_GameModeOrig (Game|GetGameMode)))
  (Variables|Default|SetPlayerHUD (Variables|/Game/Blueprints/GameLogic/PC_GameModeOrig.PC_GameModeOrig_C|GetPlayerHUD _aspc_game_mode_orig)))

(event Custom|SetHealthbarOwningChar
  ;[1 1 1 1 30] Creation
  ;;[1 1 1] Set owning character of the healthbar
  (bind _aspc_health_bar (Utilities|Casting|CastToPC_HealthBar (UserInterface|GetUserWidgetObject (Variables|Default|GetHealthBar))))
  (Default|SetOwningCharacter _aspc_health_bar self))

(event EventBeginPlay
  (CallFunction|GetHUD)
  (CallFunction|SetHealthbarOwningChar)
  (CallFunction|CreateWeapon))

(event EventTick
  (params (DeltaSeconds :type Float%20%28single-precision%29))
  (CallFunction|InteractCheck))

(event Game|Damage|EventAnyDamage
  (params (Damage :type Float%20%28single-precision%29) (DamageType :type Damage%20Type%20Object%20Reference) (InstigatedBy :type Controller%20Object%20Reference) (DamageCauser :type Actor%20Object%20Reference))
  ;[1 1 1 1 30] Damage and Death
  ;;[1 1 1] AnyDamage: Reduce health, kill character if <= 0 Health, otherwise flinch
  (bind _isalive (CallFunction|ReduceHealth Damage))
  (if _isalive
    (CallFunction|Flinch)
    (else
      (Utilities|FlowControl|DoOnce false
        (:Completed
          (CallFunction|KillCharacter))))))

(fn ConstructionScript
  (Variables|/Script/Engine.CharacterMovementComponent|SetMaxWalkSpeed (Variables|Character|GetCharacterMovement) (Variables|Default|GetWalkSpeed)))

(fn ReduceHealth
  (params (Damage :type Float%20%28single-precision%29))
  ;[1 1 1] Reduce the Character's health to a minimum of 0.
  (bind _output_get (Variables|Default|SetHealth (Math|Float|Max(Float) (- (Variables|Default|GetHealth) Damage) 0.0)))
  (bind _isalive (CallFunction|IsAlive))
  (return _output_get _isalive))

(fn IsAlive
  ;[1 1 1] True if health > 0.
  (return (> (Variables|Default|GetHealth) 0.0)))

(fn InteractCheck
  (bind _returnvalue (Transformation|GetActorLocation))
  (bind _playerhud (Variables|Default|GetPlayerHUD))
  ;[1 1 1] Cast a sphere in front of the character, and if it interacts with something implementing the Interact interface, set that as the interact actor.
  (bind _outhit (Collision|SphereTraceByChannel _returnvalue (+ _returnvalue (* (Math|Vector|GetForwardVector (Transformation|GetActorRotation)) 2e+02)) 25.0 "TraceTypeQuery2" false (Utilities|Array|MakeArray (Variables|Default|GetWeapon)) "None"))
  (if (and (.bblockinghit _outhit) (Utilities|DoesObjectImplementInterface (.hitactor _outhit) "/Game/Blueprints/UI/Dialogue/PC_I_Interactable.PC_I_Interactable_C"))
    (bind _output_get (LocalVariables|SetInteractActor (.hitactor _outhit)))
    (Default|ToggleInteractPrompt _playerhud _output_get true)
    (return (LocalVariables|GetInteractActor))
    (else
      (Default|ToggleInteractPrompt _playerhud 0 false)
      (return 0))))