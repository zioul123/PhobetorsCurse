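; Base projectile Blueprint for weapons that damages characters it overlaps and destroys itself on impact.
; Overlapping a PC_CharacterBase other than the Instigator applies fixed damage credited to the shooter's controller, then destroys the projectile.
; Overlapping the shooter is ignored, while any other overlapped actor or a blocking hit destroys it without damage.
; Destruction spawns the P_Impulse particle effect at the projectile's location.
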(event Collision|EventHit
  (params (MyComp :type Primitive%20Component%20Object%20Reference) (Other :type Actor%20Object%20Reference) (OtherComp :type Primitive%20Component%20Object%20Reference) (bSelfMoved :type Boolean) (HitLocation :type Vector :default "0, 0, 0") (HitNormal :type Vector :default "0, 0, 0") (NormalImpulse :type Vector :default "0, 0, 0") (Hit :type Hit%20Result%20Structure%20%28by%20ref%29))
  ;[1 1 1] Hit: destroy when bumping into wall
  (Actor|DestroyActor))

(event Collision|EventActorBeginOverlap
  (params (OtherActor :type Actor%20Object%20Reference))
  (bind _instigator (Variables|Actor|GetInstigator))
  ;[1 1 1] BeginOverlap: If the overlapped pawn is not the one who shot it, damage pawn, and destroy projectile
  (bind _aspc_character_base (Utilities|Casting|CastToPC_CharacterBase OtherActor)
    (:then
      (if (not (== _aspc_character_base _instigator))
        (Game|Damage|ApplyDamage _aspc_character_base 5e+01 (Pawn|GetController _instigator) self)
        (Actor|DestroyActor :!label _label)))
    (:CastFailed
      (goto _label))))

(event EventDestroyed
  ;[1 1 1] Destroyed: Play impulse effect
  (Effects|SpawnEmitteratLocation "/Game/Assets/Effects/P_Impulse.P_Impulse" (Transformation|GetActorLocation)))

(fn ConstructionScript)