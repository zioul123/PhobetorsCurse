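; Base AI controller that makes a living PC_CharacterBase pawn hunt players or wander.
; A looping timer, rather than Tick, checks pawn health and, lacking a valid Target, sphere-overlaps around the controller's location for a player-controlled character.
; With a target, it moves within the pawn's AttackRange, faces it and tries a primary attack; otherwise it moves to random navigable points.
; A debug jump event exists but its timer is disconnected.
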(event Custom|Wander
  (bind _returnvalue (Pawn|GetControlledPawn))
  ;[1 1 1] Character moves randomly
  (Utilities|IsValid _returnvalue
    (:Is%20Valid
      (AI|AIMoveTo _returnvalue (.RandomLocation (Class|NavigationSystemV1|GetRandomPointinNavigableRadius (Transformation|GetActorLocation _returnvalue) 1e+03 0 0)) 0 5.0 false))))

(event Custom|ForceJump
  (bind _returnvalue (Pawn|GetControlledPawn))
  ;[1 1 1] Just to see the character jump
  (Utilities|IsValid _returnvalue
    (:Is%20Valid
      (bind _ascharacter (Utilities|Casting|CastToCharacter _returnvalue))
      (Character|Jump _ascharacter))))

(event Custom|ProcessAI
  ;[1 1 1] If pawn is alive, check if there's a player around, then target and attack it. If there's no player around, just wander.
  (bind _isalive (CallFunction|CheckPawnIsAlive))
  (if _isalive
    (Variables|Default|GetTarget
      (:then
        (CallFunction|MoveandAttackTarget :!label _label))
      (:else
        (bind _outactors (Collision|SphereOverlapActors (Transformation|GetActorLocation) 1e+03 (Utilities|Array|MakeArray "ObjectTypeQuery3") 0 (Utilities|Array|MakeArray (Pawn|GetControlledPawn))))
        (bind _array_element (Utilities|Array|ForEachLoopwithBreak _outactors :!label _label_2)
          (:LoopBody
            (bind _aspc_character_base (Utilities|Casting|CastToPC_CharacterBase _array_element))
            (if (Class|Controller|IsPlayerController (Pawn|GetController _aspc_character_base))
              (Variables|Default|SetTarget _aspc_character_base)
              (goto _label_2 Break)))
          (:Completed
            (Variables|Default|GetTarget
              (:then
                (goto _label))
              (:else
                (CallFunction|Wander)))))))))

(event Custom|MoveAndAttackTarget
  (bind _returnvalue (Pawn|GetControlledPawn))
  ;[1 1 1] Move to the target and attack it
  (bind _target (Variables|Default|GetTarget)
    (:then
      (AI|ClearFocus)
      (AI|AIMoveTo _returnvalue "0, 0, 0" _target (Variables|/Game/Blueprints/Characters/CombatCharacters/PC_CharacterBase.PC_CharacterBase_C|GetAttackRange (.AsPC%20Character%20Base (Utilities|Casting|CastToPC_CharacterBase _returnvalue))) false
        (:OnSuccess
          (bind _aspc_character_base (Utilities|Casting|CastToPC_CharacterBase (Pawn|GetControlledPawn)))
          (AI|SetFocalPoint (Transformation|GetActorLocation (Variables|Default|GetTarget)))
          (Default|TryPrimaryAttack _aspc_character_base))))
    (:else)))

(event EventBeginPlay
  (Utilities|Time|SetTimerbyEvent (delegate Custom|ProcessAI) 2.0 true))

(event EventTick
  (params (DeltaSeconds :type Float%20%28single-precision%29)))

(fn ConstructionScript)

(fn CheckPawnIsAlive
  (bind _returnvalue (Pawn|GetControlledPawn))
  (Utilities|IsValid _returnvalue
    (:Is%20Valid
      (bind _aspc_character_base (Utilities|Casting|CastToPC_CharacterBase _returnvalue))
      (return (> (Variables|/Game/Blueprints/Characters/CombatCharacters/PC_CharacterBase.PC_CharacterBase_C|GetHealth _aspc_character_base) 0.0)))))