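; Behavior tree task that makes a boss perform its Dream Barrage attack.
; It moves the boss toward its target enemy using attack range as the acceptance radius, then triggers the barrage whether the move succeeds or fails.
; It then waits, using a barrage-specific delay for Miseria or the generic post-attack delay for other bosses, before finishing successfully.
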(event EventReceiveExecuteAI
  (params (OwnerController :type AI%20Controller%20Object%20Reference) (ControlledPawn :type Pawn%20Object%20Reference))
  (bind _aspc_bp_enemy_boss (Utilities|Casting|CastToPC_BP_EnemyBoss ControlledPawn))
  (AI|AIMoveTo _aspc_bp_enemy_boss "0, 0, 0" (Variables|/Game/Blueprints/Actors/CombatCharacters/PC_BP_EnemyBoss.PC_BP_EnemyBoss_C|GetTargetEnemy _aspc_bp_enemy_boss) (Variables|/Game/Blueprints/Actors/CombatCharacters/PC_BP_Character.PC_BP_Character_C|GetAttackRange _aspc_bp_enemy_boss) false
    (:OnSuccess
      _)
    (:OnFail
      _))
  (Default|TryDreamBarrage _aspc_bp_enemy_boss)
  (bind _aspc_bp_miseria (Utilities|Casting|CastToPC_BP_Miseria _aspc_bp_enemy_boss)
    (:then
      (Utilities|FlowControl|Delay (Variables|/Game/Blueprints/Actors/CombatCharacters/PC_BP_Miseria.PC_BP_Miseria_C|GetDreamBarrageDelayAfter _aspc_bp_miseria)))
    (:CastFailed
      (Utilities|FlowControl|Delay (Variables|/Game/Blueprints/Actors/CombatCharacters/PC_BP_Enemy.PC_BP_Enemy_C|GetDelayAfterAttack _aspc_bp_enemy_boss))))
  (AI|BehaviorTree|FinishExecute true))