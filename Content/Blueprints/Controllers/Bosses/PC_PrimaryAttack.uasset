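; PC_PrimaryAttack is a behavior tree task that makes an enemy boss approach its target and perform a primary attack.
; On execution it moves the controlled PC_BP_EnemyBoss toward its TargetEnemy, using the boss's AttackRange as the acceptance radius.
; A successful move triggers TryPrimaryAttack.
; Both success and failure then wait for the boss's DelayAfterAttack and finish the task as successful.
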(event EventReceiveExecuteAI
  (params (OwnerController :type AI%20Controller%20Object%20Reference) (ControlledPawn :type Pawn%20Object%20Reference))
  (bind _aspc_bp_enemy_boss (Utilities|Casting|CastToPC_BP_EnemyBoss ControlledPawn))
  ;[1 1 1] Move to the target and attack it
  (Development|PrintString "PC_PrimaryAttack: Moving to attack")
  (bind _output_get (Variables|Default|SetControlledEnemy _aspc_bp_enemy_boss))
  (AI|AIMoveTo _output_get "0, 0, 0" (Variables|/Game/Blueprints/Actors/CombatCharacters/PC_BP_EnemyBoss.PC_BP_EnemyBoss_C|GetTargetEnemy _aspc_bp_enemy_boss) (Variables|/Game/Blueprints/Actors/CombatCharacters/PC_BP_Character.PC_BP_Character_C|GetAttackRange (Variables|Default|GetControlledEnemy)) false
    (:OnSuccess
      (Default|TryPrimaryAttack (Variables|Default|GetControlledEnemy)))
    (:OnFail
      _))
  (Utilities|FlowControl|Delay (Variables|/Game/Blueprints/Actors/CombatCharacters/PC_BP_Enemy.PC_BP_Enemy_C|GetDelayAfterAttack (Variables|Default|GetControlledEnemy)))
  (AI|BehaviorTree|FinishExecute true))