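; Behavior tree task for the Elina stalker AI that records whether an Elina Somnia character is within kill range.
; On execute it ends stalking, runs a pawn sphere overlap around the stalker's capsule using its KillRange, writes the result to a Blackboard bool, prints it and finishes successfully.
; A helper that compares target distance to LoseAggroRange is defined but not called in the event graph.
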(event EventReceiveExecuteAI
  (params (OwnerController :type AI%20Controller%20Object%20Reference) (ControlledPawn :type Pawn%20Object%20Reference))
  (bind _aspc_bp_elina_stalker (Utilities|Casting|CastToPC_BP_ElinaStalker ControlledPawn))
  (Default|EndStalking _aspc_bp_elina_stalker)
  (bind _outactors (Collision|SphereOverlapActors (Transformation|GetWorldLocation (Variables|/Script/Engine.Character|GetCapsuleComponent _aspc_bp_elina_stalker)) (Variables|/Game/Blueprints/Actors/CombatCharacters/PC_BP_ElinaStalker.PC_BP_ElinaStalker_C|GetKillRange _aspc_bp_elina_stalker) (Utilities|Array|MakeArray "ObjectTypeQuery3") "/Game/Blueprints/Actors/CombatCharacters/PC_BP_ElinaSomnia.PC_BP_ElinaSomnia_C"))
  (Class|BTFunctionLibrary|SetBlackboardValueasBool (Variables|Default|GetBB_hasCharacterNearby) (> (Utilities|Array|Length _outactors) 0))
  (Development|PrintString (Utilities|String|Append "SetCharacterNearby: " (Utilities|String|ToString(Boolean) (> (Utilities|Array|Length _outactors) 0))))
  (AI|BehaviorTree|FinishExecute true))

(fn IsTargetStillClose
  (params (Target :type PC%20BP%20Character%20Object%20Reference) (ControlledPawn :type PC%20BP%20Enemy%20Object%20Reference))
  (return (<= (Math|Vector|Distance(Vector) (Transformation|GetWorldLocation (Variables|/Script/Engine.Character|GetCapsuleComponent Target)) (Transformation|GetWorldLocation (Variables|/Script/Engine.Character|GetCapsuleComponent ControlledPawn))) (Variables|/Game/Blueprints/Actors/CombatCharacters/PC_BP_Enemy.PC_BP_Enemy_C|GetLoseAggroRange ControlledPawn))))