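; Behavior tree decorator for enemy AI that passes when the BBHasCharacterNearby blackboard bool is true.
; On execution start, it runs a sphere overlap for pawns within the controlled PC_EnemyBase's AggroRange, ignoring itself.
; It checks overlapped PC_CharacterBase actors for player control, but that branch is empty.
; The blackboard value is only read here, so the scan does not affect the condition.
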(event EventReceiveExecutionStartAI
  (params (OwnerController :type AI%20Controller%20Object%20Reference) (ControlledPawn :type Pawn%20Object%20Reference))
  (bind _aspc_enemy_base (Utilities|Casting|CastToPC_EnemyBase ControlledPawn))
  (bind _outactors (Collision|SphereOverlapActors (Transformation|GetActorLocation _aspc_enemy_base) (Variables|/Game/Blueprints/Actors/Old/CombatCharacters/PC_EnemyBase.PC_EnemyBase_C|GetAggroRange _aspc_enemy_base) (Utilities|Array|MakeArray "ObjectTypeQuery3") 0 (Utilities|Array|MakeArray ControlledPawn)))
  (bind _array_element (Utilities|Array|ForEachLoopwithBreak _outactors)
    (:LoopBody
      (bind _aspc_character_base (Utilities|Casting|CastToPC_CharacterBase _array_element))
      (if (Pawn|IsPlayerControlled _aspc_character_base)
        _))))

(fn PerformConditionCheckAI
  (params (OwnerController :type AI%20Controller%20Object%20Reference) (ControlledPawn :type Pawn%20Object%20Reference))
  (return (Class|BTFunctionLibrary|GetBlackboardValueasBool (Variables|Default|GetBB_hasCharacterNearby))))