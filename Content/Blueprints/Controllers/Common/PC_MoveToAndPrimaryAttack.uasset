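; Behavior tree task that sends an enemy to its blackboard target and triggers its primary attack.
; It flags the controlled enemy as aggro, then moves toward the target actor using the enemy's attack range as the acceptance radius.
; On arrival it tries the primary attack; success or failed move both wait the enemy's post-attack delay, then finish the task as successful.
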(event EventReceiveExecuteAI
  (params (OwnerController :type AI%20Controller%20Object%20Reference) (ControlledPawn :type Pawn%20Object%20Reference))
  (bind _aspc_bp_enemy (Utilities|Casting|CastToPC_BP_Enemy ControlledPawn))
  ;[1 1 1] Move to the target and attack it
  (Development|PrintString "PC_MoveToAndPrimaryAttack: Moving to attack")
  (Variables|/Game/Blueprints/Actors/CombatCharacters/PC_BP_Enemy.PC_BP_Enemy_C|SetCurrentlyAggro _aspc_bp_enemy true)
  (bind _output_get (Variables|Default|SetControlledEnemy _aspc_bp_enemy))
  (AI|AIMoveTo _output_get "0, 0, 0" (.AsActor (Utilities|Casting|CastToActor (Class|BTFunctionLibrary|GetBlackboardValueasObject (Variables|Default|GetBB_Target)))) (Variables|/Game/Blueprints/Actors/CombatCharacters/PC_BP_Character.PC_BP_Character_C|GetAttackRange (Variables|Default|GetControlledEnemy)) false
    (:OnSuccess
      (Default|TryPrimaryAttack (Variables|Default|GetControlledEnemy)))
    (:OnFail
      _))
  (Utilities|FlowControl|Delay (Variables|/Game/Blueprints/Actors/CombatCharacters/PC_BP_Enemy.PC_BP_Enemy_C|GetDelayAfterAttack (Variables|Default|GetControlledEnemy)))
  (AI|BehaviorTree|FinishExecute true))