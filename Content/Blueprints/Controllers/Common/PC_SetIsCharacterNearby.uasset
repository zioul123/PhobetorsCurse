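; Behavior Tree task that checks whether a player-controlled character is within an enemy's aggro range.
; It resets the nearby-character Blackboard flag and clears the enemy's CurrentlyAggro state, then runs a pawn sphere overlap at AggroRange, drawn with a debug sphere.
; The first player-controlled PC_BP_Character found becomes the Blackboard target and sets the flag, leaving the target untouched when none is found.
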(event EventReceiveExecuteAI
  (params (OwnerController :type AI%20Controller%20Object%20Reference) (ControlledPawn :type Pawn%20Object%20Reference))
  ;[1 1 1] Cast a sphere overlap around the enemy, change the BB values to the target and hasCharacterNearby if there are playere controlled pawns nearby.
  (Class|BTFunctionLibrary|SetBlackboardValueasBool (Variables|Default|GetBB_hasCharacterNearby) false) ; First reset BB value. The For loop will flip this to true if possible.
  (bind _aspc_bp_enemy (Utilities|Casting|CastToPC_BP_Enemy ControlledPawn))
  (Variables|/Game/Blueprints/Actors/CombatCharacters/PC_BP_Enemy.PC_BP_Enemy_C|SetCurrentlyAggro _aspc_bp_enemy false)
  (Rendering|Debug|DrawDebugSphere (Transformation|GetActorLocation _aspc_bp_enemy) (Variables|/Game/Blueprints/Actors/CombatCharacters/PC_BP_Enemy.PC_BP_Enemy_C|GetAggroRange _aspc_bp_enemy) 12 "(R=1.000000,G=1.000000,B=1.000000,A=1.000000)" 2.0)
  (bind _outactors (Collision|SphereOverlapActors (Transformation|GetActorLocation _aspc_bp_enemy) (Variables|/Game/Blueprints/Actors/CombatCharacters/PC_BP_Enemy.PC_BP_Enemy_C|GetAggroRange _aspc_bp_enemy) (Utilities|Array|MakeArray "ObjectTypeQuery3") 0 (Utilities|Array|MakeArray 0)))
  (bind _array_element (Utilities|Array|ForEachLoopwithBreak _outactors :!label _label)
    (:LoopBody
      (bind _aspc_bp_character (Utilities|Casting|CastToPC_BP_Character _array_element))
      (if (Pawn|IsPlayerControlled _aspc_bp_character)
        (Class|BTFunctionLibrary|SetBlackboardValueasObject (Variables|Default|GetBB_Target) _aspc_bp_character)
        (Class|BTFunctionLibrary|SetBlackboardValueasBool (Variables|Default|GetBB_hasCharacterNearby) true)
        (goto _label Break)))
    (:Completed
      (AI|BehaviorTree|FinishExecute true))))